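; Spider enemy that chases the player and deals melee damage through a hitbox toggled by attack events.
; A looping timer refreshes the navmesh path, which Tick follows with manual movement input while IsMoving is set.
; Tick also mirrors the damage component's health and stun state to the health bar, AnimBP and stun VFX.
; Hits flash the materials and spawn damage numbers; death scatters mana droplets.
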(event `self.ReceiveTick`
  (params (DeltaSeconds :type "Float (single-precision)"))
  (bind _returnvalue (`self.K2_GetActorLocation`))
  (bind _bpc_dmgsys (`self.BPC_dmgSys`))
  (bind _mesh (`self.Mesh`))
  (bind _stunsystem (`self.stunSystem`))
  (bind _path_points (`self.Path Points`))
  (bind _pathindex (`self.PathIndex`))
  (bind _output (`|GetArrayItem` _path_points _pathindex))
  (bind _stunned (`/Game/HPSystem/BPC_dmgSys.stunned` (`self.BPC_dmgSys`)))
  (bind _aswbp_health_bar (cast `/Game/Characters/Enemy/WBP_HealthBar` (`WidgetComponent.GetWidget` (`self.Health`))))
  (set `/Game/Characters/Enemy/WBP_HealthBar.HealthPercent` (/ (`/Game/HPSystem/BPC_dmgSys.health` _bpc_dmgsys) (`/Game/HPSystem/BPC_dmgSys.maxHealth` _bpc_dmgsys)) _aswbp_health_bar)
  (if _stunned
    (bind _asanim_bp_bad_spida (cast `/Game/Characters/BadSpider/AnimBP_BadSpida` (`SkeletalMeshComponent.GetAnimInstance` (`self.Mesh`))))
    (if (and _stunned (not (`/Game/Characters/BadSpider/AnimBP_BadSpida.stunned` _asanim_bp_bad_spida)))
      (bind _returnvalue_2 (`NiagaraFunctionLibrary.SpawnSystemAttached` "/Game/HPSystem/NS_Stun.NS_Stun" (`self.Mesh`) "None" (0.0 40.0 300.0) (struct) "KeepRelativeOffset" true))
      (set `self.stunSystem` _returnvalue_2))
    (set `self.speedScale` 0.0)
    (bind _asanim_bp_bad_spida_2 (cast `/Game/Characters/BadSpider/AnimBP_BadSpida` (`SkeletalMeshComponent.GetAnimInstance` (`self.Mesh`))))
    (set `/Game/Characters/BadSpider/AnimBP_BadSpida.stunned` true _asanim_bp_bad_spida_2)
    (else
      (if (`KismetSystemLibrary.IsValid` _stunsystem)
        (`ActorComponent.K2_DestroyComponent` _stunsystem))
      (set `self.speedScale` 0.8)
      (bind _asanim_bp_bad_spida_3 (cast `/Game/Characters/BadSpider/AnimBP_BadSpida` (`SkeletalMeshComponent.GetAnimInstance` (`self.Mesh`))))
      (set `/Game/Characters/BadSpider/AnimBP_BadSpida.stunned` false _asanim_bp_bad_spida_3)))
  (if (> (- (`KismetSystemLibrary.GetGameTimeInSeconds`) (`self.lastDamageTakeTime`)) 0.2)
    (for _index (range (`PrimitiveComponent.GetNumMaterials` _mesh))
      (`PrimitiveComponent.SetMaterial` _mesh _index (`|GetArrayItem` (`self.OGMats`) _index))))
  (bind _asanim_bp_bad_spida_4 (cast `/Game/Characters/BadSpider/AnimBP_BadSpida` (`SkeletalMeshComponent.GetAnimInstance` (`self.Mesh`))))
  (`SceneComponent.SetVisibility` (`self.ExclamationMark`) (or (`self.isMoving`) (`/Game/Characters/BadSpider/AnimBP_BadSpida.CanAttack` _asanim_bp_bad_spida_4)) false)
  (if (`self.isMoving`)
    (if (< _pathindex (`KismetArrayLibrary.Array_Length` _path_points))
      (`self.AddMovementInput` (`KismetMathLibrary.Normal` (`KismetMathLibrary.MakeVector` (.x (- _output _returnvalue)) (.y (- _output _returnvalue)))) (* DeltaSeconds 80.0))
      (if (< (`KismetMathLibrary.Vector_Distance` _returnvalue _output) 100.0)
        (`/Engine/EditorBlueprintResources/StandardMacros.IncrementInt` (`self.PathIndex`))))))

(event `StartAttack`
  (`AudioComponent.Play` (`self.AttackAudio`) 0.2)
  (`PrimitiveComponent.SetCollisionEnabled` (`self.Melee_Hitbox`) "QueryOnly"))

(event `EndAttack`
  (`PrimitiveComponent.SetCollisionEnabled` (`self.Melee_Hitbox`) "NoCollision"))

(event `self.ReceiveBeginPlay`
  (bind _mesh (`self.Mesh`))
  (`KismetSystemLibrary.K2_SetTimerDelegate` (delegate `Repath`) 0.1 true true)
  (for _index (range (`PrimitiveComponent.GetNumMaterials` _mesh))
    (`KismetArrayLibrary.Array_Add` (`self.OGMats`) (`PrimitiveComponent.GetMaterial` _mesh _index)))
  (set `self.FlashMat` "/Game/HPSystem/FlashMat.FlashMat")
  (bind _asbp_third_person_character (cast `/Game/ThirdPerson/Blueprints/BP_ThirdPersonCharacter` (`GameplayStatics.GetPlayerCharacter` 0)))
  (set `self.PlayerRef_0` _asbp_third_person_character))

(event `Repath`
  (bind _returnvalue (`NavigationSystemV1.FindPathToLocationSynchronously` (`self.K2_GetActorLocation`) (`NavigationSystemV1.K2_ProjectPointToNavigation` (`self.K2_GetActorLocation` (`self.PlayerRef_0`)) null null (1000.0 1000.0 1000.0)) null null))
  (bind _pathpoints (`NavigationPath.PathPoints` _returnvalue))
  (if (> (`KismetArrayLibrary.Array_Length` _pathpoints) 0)
    (set `self.Path Points` _pathpoints)
    (set `self.PathIndex` 1)))

(event `self.BPC_dmgSys.onDeath`
  (bind _returnvalue (`self.K2_GetActorLocation`))
  (`KismetSystemLibrary.DelayUntilNextTick`)
  (`NiagaraFunctionLibrary.SpawnSystemAtLocation` "/Game/Characters/Enemy/NS_EnemyDeath.NS_EnemyDeath" _returnvalue)
  (for _ (range 5)
    (bind _returnvalue_2 (`|SpawnActorFromClass` "/Game/Spells/BP_ManaDroplet.BP_ManaDroplet_C" (`KismetMathLibrary.Conv_VectorToTransform` _returnvalue) "AlwaysSpawn" "MultiplyWithRoot" null null))
    (`/Engine/EditorBlueprintResources/StandardMacros.IsValid` _returnvalue_2
      (:`Is Valid`
        (`PrimitiveComponent.AddImpulse` (`/Game/Spells/BP_ManaDroplet.Sphere` _returnvalue_2) (* (`KismetMathLibrary.RandomUnitVector`) 5.0) "None" false))))
  (`self.K2_DestroyActor`))

(event `self.Melee_Hitbox.OnComponentBeginOverlap`
  (params (OverlappedComponent :type "PrimitiveComponent Object Reference") (OtherActor :type "Actor Object Reference") (OtherComp :type "PrimitiveComponent Object Reference") (OtherBodyIndex :type Integer) (bFromSweep :type Boolean) (SweepResult :type "HitResult Structure (by ref)"))
  (bind _asbp_third_person_character (cast `/Game/ThirdPerson/Blueprints/BP_ThirdPersonCharacter` OtherActor))
  (bind _wasdamaged (`/Game/HPSystem/dmgSystem.doReceiveDamage` _asbp_third_person_character (`self.DamageDealt`) "NewEnumerator1" "NewEnumerator1" 0.0))
  (if _wasdamaged
    (set `self.lastHitTIme` (`KismetSystemLibrary.GetGameTimeInSeconds`))
    (`PrimitiveComponent.SetCollisionEnabled` (`self.Melee_Hitbox`) "NoCollision")))

(fn `doReceiveDamage`
  (params (dmgAmount :type "Float (double-precision)") (dmgResponse :type "/Game/HPSystem/dmgResponse Enum" :default "NewEnumerator0") (dmgType :type "/Game/HPSystem/dmgType Enum" :default "NewEnumerator0") (responseDuration :type "Float (double-precision)"))
  (returns (wasDamaged :type Boolean))
  (bind _mesh (`self.Mesh`))
  (`self.PlayHurtSound`)
  (bind _wasdamaged (`/Game/HPSystem/BPC_dmgSys.takeDamage` (`self.BPC_dmgSys`) dmgAmount dmgResponse dmgType responseDuration))
  (bind _returnvalue (`|SpawnActorFromClass` "/Game/Characters/Enemy/BP_DamageNumber.BP_DamageNumber_C" (`SceneComponent.K2_GetComponentToWorld` (`self.ExclamationMark`)) "Undefined" "MultiplyWithRoot" null null))
  (bind _aswbp_damage_number (cast `/Game/Characters/Enemy/WBP_DamageNumber` (`WidgetComponent.GetWidget` (`/Game/Characters/Enemy/BP_DamageNumber.Number` _returnvalue))))
  (set `/Game/Characters/Enemy/WBP_DamageNumber.Damage` dmgAmount _aswbp_damage_number)
  (if (> (- (`KismetSystemLibrary.GetGameTimeInSeconds`) (`self.lastDamageTakeTime`)) 0.2)
    (set `self.lastDamageTakeTime` (`KismetSystemLibrary.GetGameTimeInSeconds`))
    (for _index (range (`PrimitiveComponent.GetNumMaterials` _mesh))
      (`PrimitiveComponent.SetMaterial` _mesh _index (`self.FlashMat`))))
  (return _wasdamaged))

(fn `UserConstructionScript`)