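; Enemy character Blueprint that can take damage, be healed and be stunned.
; Damage, healing and health queries are forwarded to the BPCDmgSys component, while DoReceiveEffect is a stub that always returns false.
; Tick polls the component's Stunned flag to deactivate or reactivate CharacterMovement.
; Two events apply or clear an overlay material on the mesh.
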(event `self.ReceiveTick`
  (params (DeltaSeconds :type "Float (single-precision)"))
  (bind _charactermovement (`self.CharacterMovement`))
  (if (`/Game/HPSystem/BPC_dmgSys.stunned` (`self.BPC_dmgSys`))
    (`ActorComponent.Deactivate` _charactermovement)
    (else
      (`ActorComponent.Activate` _charactermovement false))))

(event `/Game/HPSystem/dmgSystem.doApplyOverlayMaterial`
  (params (OverlayMaterial :type "Material Object Reference") (EffectClass :type "/Game/HPSystem/Effects/BP_BaseEffect Class Reference"))
  (`MeshComponent.SetOverlayMaterial` (`self.Mesh`) OverlayMaterial))

(event `/Game/HPSystem/dmgSystem.doRemoveOverlayMaterial`
  (params (EffectClass :type "/Game/HPSystem/Effects/BP_BaseEffect Class Reference"))
  (`MeshComponent.SetOverlayMaterial` (`self.Mesh`) null))

(fn `doHeal`
  (params (healAmount :type "Float (double-precision)"))
  (returns (newHealth :type "Float (double-precision)"))
  (bind _newhealth (`/Game/HPSystem/BPC_dmgSys.heal` (`self.BPC_dmgSys`) healAmount))
  (return _newhealth))

(fn `doReceiveDamage`
  (params (dmgAmount :type "Float (double-precision)") (dmgResponse :type "/Game/HPSystem/dmgResponse Enum" :default "NewEnumerator0") (dmgType :type "/Game/HPSystem/dmgType Enum" :default "NewEnumerator0") (responseDuration :type "Float (double-precision)"))
  (returns (wasDamaged :type Boolean))
  (bind _wasdamaged (`/Game/HPSystem/BPC_dmgSys.takeDamage` (`self.BPC_dmgSys`) dmgAmount dmgResponse dmgType responseDuration))
  (return _wasdamaged))

(fn `doReceiveEffect`
  (params (EffectData :type "/Game/HPSystem/Effects/PDA_effectData Object Reference"))
  (returns (WasAffected :type Boolean))
  (return false))

(fn `getHealth`
  (returns (health :type "Float (double-precision)"))
  (return (`/Game/HPSystem/BPC_dmgSys.health` (`self.BPC_dmgSys`))))

(fn `getMaxHealth`
  (returns (maxHealth :type "Float (double-precision)"))
  (return (`/Game/HPSystem/BPC_dmgSys.maxHealth` (`self.BPC_dmgSys`))))

(fn `UserConstructionScript`)