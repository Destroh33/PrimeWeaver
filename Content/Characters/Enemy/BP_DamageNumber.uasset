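; Floating damage number actor for enemy hits, showing a WBP_DamageNumber through its Number widget component.
; Every tick it rotates to face the player camera, rises at a steady rate and advances a timer.
; Over Duration it linearly fades the widget's opacity and shrinks the actor's scale to zero, then destroys itself.
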(event `self.ReceiveTick`
  (params (DeltaSeconds :type "Float (single-precision)"))
  (bind _returnvalue (`KismetMathLibrary.Lerp` 1.0 0.0 (/ (`self.Timer`) (`self.Duration`))))
  (`self.K2_SetActorRotation` (`KismetMathLibrary.FindLookAtRotation` (`self.K2_GetActorLocation`) (`PlayerCameraManager.GetCameraLocation` (`PlayerController.PlayerCameraManager` (`GameplayStatics.GetPlayerController` 0)))))
  (bind _output_get (set `self.Timer` (+ (`self.Timer`) DeltaSeconds)))
  (if (> _output_get (`self.Duration`))
    (`self.K2_DestroyActor`)
    (else
      (bind _output_get_2 (set `self.Opacity` _returnvalue))
      (bind _aswbp_damage_number (cast `/Game/Characters/Enemy/WBP_DamageNumber` (`WidgetComponent.GetWidget` (`self.Number`))))
      (set `/Game/Characters/Enemy/WBP_DamageNumber.Opacity` _output_get_2 _aswbp_damage_number)
      (`self.K2_SetActorLocation` (`KismetMathLibrary.MakeVector` (.x (`self.K2_GetActorLocation`)) (.y (`self.K2_GetActorLocation`)) (+ (.z (`self.K2_GetActorLocation`)) (* DeltaSeconds 100.0))))
      (`self.SetActorScale3D` (`KismetMathLibrary.MakeVector` _returnvalue _returnvalue _returnvalue)))))

(fn `UserConstructionScript`)