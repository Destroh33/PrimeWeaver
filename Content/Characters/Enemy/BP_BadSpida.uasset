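; BP_BadSpida is an enemy character Blueprint that can take damage and be healed.
; It delegates health logic to a BPCDmgSys damage-system component, forwarding heal amounts and damage amount, response and type, then returning the results.
; Health and max health getters read straight from that component, and the construction script is empty.
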(fn `doHeal`
  (params (healAmount :type "Float (double-precision)"))
  (returns (newHealth :type "Float (double-precision)"))
  (bind _newhealth (`/Game/HPSystem/BPC_dmgSys.heal` (`self.BPC_dmgSys`) healAmount))
  (return _newhealth))

(fn `doReceiveDamage`
  (params (dmgAmount :type "Float (double-precision)") (dmgResponse :type "/Game/HPSystem/dmgResponse Enum" :default "NewEnumerator0") (dmgType :type "/Game/HPSystem/dmgType Enum" :default "NewEnumerator0"))
  (returns (wasDamaged :type Boolean))
  (bind _wasdamaged (`/Game/HPSystem/BPC_dmgSys.takeDamage` (`self.BPC_dmgSys`) dmgAmount dmgResponse dmgType))
  (return _wasdamaged))

(fn `getHealth`
  (returns (health :type "Float (double-precision)"))
  (return (`/Game/HPSystem/BPC_dmgSys.health` (`self.BPC_dmgSys`))))

(fn `getMaxHealth`
  (returns (maxHealth :type "Float (double-precision)"))
  (return (`/Game/HPSystem/BPC_dmgSys.maxHealth` (`self.BPC_dmgSys`))))

(fn `UserConstructionScript`)