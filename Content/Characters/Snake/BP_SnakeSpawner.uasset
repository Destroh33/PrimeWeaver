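; BP_SnakeSpawner is a looping snake hazard that warns with a widget, then rotates and deals heavy damage on hit to the player character or enemies.
; A self-calling SpawnSnake event, started on BeginPlay, shows the warning at the ExclamationLoc actor, enables movement for a set duration, then resets and waits.
; While moving, Tick rolls the Scene component at a constant rate.
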(event `self.ReceiveBeginPlay`
  (`self.SpawnSnake` (`self.Timebetweensnakes`))
  (`SceneComponent.K2_SetWorldLocation` (`self.Widget`) (`self.K2_GetActorLocation` (`self.Exclamation Loc`)) false false))

(event `self.ReceiveHit`
  (params (MyComp :type "PrimitiveComponent Object Reference") (Other :type "Actor Object Reference") (OtherComp :type "PrimitiveComponent Object Reference") (bSelfMoved :type Boolean) (HitLocation :type "Vector Structure") (HitNormal :type "Vector Structure") (NormalImpulse :type "Vector Structure") (Hit :type "HitResult Structure (by ref)"))
  (bind _asbp_third_person_character (cast `/Game/ThirdPerson/Blueprints/BP_ThirdPersonCharacter` Other)
    (:`then`
      (`/Game/ThirdPerson/Blueprints/BP_ThirdPersonCharacter.doReceiveDamage` _asbp_third_person_character 500.0 "NewEnumerator1" "NewEnumerator2" 0.0))
    (:`CastFailed`
      (bind _asbp_enemy (cast `/Game/Characters/Enemy/BP_Enemy` Other))
      (`/Game/Characters/Enemy/BP_Enemy.doReceiveDamage` _asbp_enemy 500.0 "NewEnumerator1" "NewEnumerator2" 0.0))))

(event `self.ReceiveTick`
  (params (DeltaSeconds :type "Float (single-precision)"))
  (bind _scene (`self.Scene`))
  (if (`self.isMoving`)
    (`SceneComponent.K2_SetRelativeRotation` _scene (`KismetMathLibrary.MakeRotator` (+ (* DeltaSeconds -100.0) (.roll (`SceneComponent.RelativeRotation` _scene))) (.pitch (`SceneComponent.RelativeRotation` _scene)) (.yaw (`SceneComponent.RelativeRotation` _scene))) false false)))

(event `SpawnSnake`
  (params (timeTillNext :type "Float (double-precision)"))
  (bind _widget (`self.Widget`))
  (`SceneComponent.SetVisibility` _widget true false)
  (`KismetSystemLibrary.Delay` (`self.warningtime`))
  (set `self.isMoving` true)
  (`SceneComponent.SetVisibility` _widget false false)
  (`KismetSystemLibrary.Delay` (`self.duration`))
  (`SceneComponent.K2_SetRelativeRotation` :`self` (`self.Scene`))
  (set `self.isMoving` false)
  (`KismetSystemLibrary.Delay` timeTillNext)
  (`self.SpawnSnake` (`self.Timebetweensnakes`)))

(fn `UserConstructionScript`)