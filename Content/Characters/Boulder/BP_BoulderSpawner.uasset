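; BP_BoulderSpawner is a spawner actor that continuously emits BP_Boulder actors from its own transform.
; BeginPlay starts a custom event that calls SpawnBoulder, waits a configurable interval, then calls itself again to loop indefinitely.
; SpawnBoulder multiplies each new boulder's scale by a size variable and sets its lifespan so it cleans itself up.
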(event `SpawnBoulderEvent`
  (`self.SpawnBoulder` (`self.boulder lifeteime`))
  (`KismetSystemLibrary.Delay` (`self.time between boulders`))
  (`self.SpawnBoulderEvent`))

(event `self.ReceiveBeginPlay`
  (`self.SpawnBoulderEvent`))

(fn `SpawnBoulder`
  (params (BoulderLifetime :type "Float (double-precision)"))
  (bind _returnvalue (`|SpawnActorFromClass` "/Game/Characters/Boulder/BP_Boulder.BP_Boulder_C" (`self.GetTransform`) "Undefined" "MultiplyWithRoot" null null))
  (`self.SetActorScale3D` _returnvalue (* (`self.GetActorScale3D` _returnvalue) (`self.bouldersize`)))
  (`self.SetLifeSpan` _returnvalue BoulderLifetime))

(fn `UserConstructionScript`)