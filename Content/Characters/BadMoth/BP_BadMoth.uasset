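; BP_BadMoth is a bobbing enemy that faces the player in range and fires BP_MothProjectile every two seconds.
; Tick drives sine hovering and lerped rotation, creeping toward the player only when InArena; the timer-refreshed nav path is never followed.
; DoReceiveDamage forwards hits to the damage component, spawning damage numbers and briefly swapping materials to flash.
; OnDeath spawns an effect and scattered mana droplets, then destroys the moth.
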(event `self.ReceiveBeginPlay`
  (bind _skeletalmesh (`self.SkeletalMesh`))
  (`KismetSystemLibrary.K2_SetTimerDelegate` (delegate `Repath`) 0.1 true true)
  (for _index (range (`PrimitiveComponent.GetNumMaterials` _skeletalmesh))
    (`KismetArrayLibrary.Array_Add` (`self.OGMats`) (`PrimitiveComponent.GetMaterial` _skeletalmesh _index)))
  (set `self.FlashMat` "/Game/HPSystem/FlashMat.FlashMat")
  (bind _asbp_third_person_character (cast `/Game/ThirdPerson/Blueprints/BP_ThirdPersonCharacter` (`GameplayStatics.GetPlayerCharacter` 0)))
  (set `self.Player Ref` _asbp_third_person_character)
  (set `self.StartZ` (.z (`self.K2_GetActorLocation`))))

(event `Repath`
  (bind _returnvalue (`NavigationSystemV1.FindPathToLocationSynchronously` (`self.K2_GetActorLocation`) (`NavigationSystemV1.K2_ProjectPointToNavigation` (`self.K2_GetActorLocation` (`self.Player Ref`)) null null (1000.0 1000.0 1000.0)) null null))
  (bind _pathpoints (`NavigationPath.PathPoints` _returnvalue))
  (if (> (`KismetArrayLibrary.Array_Length` _pathpoints) 0)
    (set `self.Path Points` _pathpoints)
    (set `self.Path Index` 1)))

(event `self.ReceiveTick`
  (params (DeltaSeconds :type "Float (single-precision)"))
  (bind _returnvalue (`self.K2_GetActorLocation`))
  (bind _player_ref (`self.Player Ref`))
  (bind _bpc_dmgsys (`self.BPC_dmgSys`))
  (bind _skeletalmesh (`self.SkeletalMesh`))
  (bind _returnvalue_2 (`SceneComponent.GetSocketLocation` (`self.SkeletalMesh`) "shoot_Socket"))
  (bind _aswbp_health_bar (cast `/Game/Characters/Enemy/WBP_HealthBar` (`WidgetComponent.GetWidget` (`self.Health`)))
    (:`then`
      (set `/Game/Characters/Enemy/WBP_HealthBar.HealthPercent` (/ (`/Game/HPSystem/BPC_dmgSys.health` _bpc_dmgsys) (`/Game/HPSystem/BPC_dmgSys.maxHealth` _bpc_dmgsys)) _aswbp_health_bar))
    (:`CastFailed`
      _))
  (if (> (- (`KismetSystemLibrary.GetGameTimeInSeconds`) (`self.lastDamageTakeTime`)) 0.2)
    (for _index (range (`PrimitiveComponent.GetNumMaterials` _skeletalmesh))
      (`PrimitiveComponent.SetMaterial` _skeletalmesh _index (`|GetArrayItem` (`self.OGMats`) _index))))
  (set `MovementComponent.Velocity` (0.0 0.0 0.0) (`self.CharacterMovement`))
  (`SceneComponent.SetVisibility` (`self.ExclamationMark`) (`self.InRange`) false)
  (bind _output_get (set `self.TimePassed` (+ (`self.TimePassed`) DeltaSeconds)))
  (`self.K2_SetActorLocation` (`KismetMathLibrary.MakeVector` (.x _returnvalue) (.y _returnvalue) (+ (`self.StartZ`) (* (`KismetMathLibrary.DegSin` (* _output_get 445.0)) 15.0))))
  (bind _output_get_2 (set `self.InRange` (< (`self.GetDistanceTo` _player_ref) (select `bool` (`self.inArena`) :`false` 1500.0 :`true` 10000.0))))
  (if _output_get_2
    (`self.K2_SetActorLocationAndRotation` (`KismetMathLibrary.MakeVector` (.x (`KismetMathLibrary.VLerp` (`KismetMathLibrary.MakeVector` (.x (`self.K2_GetActorLocation`)) (.y (`self.K2_GetActorLocation`))) (`KismetMathLibrary.MakeVector` (.x (select `bool` (`self.inArena`) :`false` (`self.K2_GetActorLocation`) :`true` (`self.K2_GetActorLocation` (`self.Player Ref`)))) (.y (select `bool` (`self.inArena`) :`false` (`self.K2_GetActorLocation`) :`true` (`self.K2_GetActorLocation` (`self.Player Ref`))))) 0.002)) (.y (`KismetMathLibrary.VLerp` (`KismetMathLibrary.MakeVector` (.x (`self.K2_GetActorLocation`)) (.y (`self.K2_GetActorLocation`))) (`KismetMathLibrary.MakeVector` (.x (select `bool` (`self.inArena`) :`false` (`self.K2_GetActorLocation`) :`true` (`self.K2_GetActorLocation` (`self.Player Ref`)))) (.y (select `bool` (`self.inArena`) :`false` (`self.K2_GetActorLocation`) :`true` (`self.K2_GetActorLocation` (`self.Player Ref`))))) 0.002)) (.z (`self.K2_GetActorLocation`))) (`KismetMathLibrary.RLerp` (`self.K2_GetActorRotation`) (`KismetMathLibrary.MakeRotator` 0.0 0.0 (.yaw (`KismetMathLibrary.FindLookAtRotation` _returnvalue (`self.K2_GetActorLocation` _player_ref)))) 0.1 true))
    (if (> (- (`KismetSystemLibrary.GetGameTimeInSeconds`) (`self.LastAttackTime`)) 2.0)
      (`|PlayMontage` (`self.SkeletalMesh`) "/Game/Characters/BadMoth/AM_BadMothAttack.AM_BadMothAttack"
        (:`then`
          (set `self.LastAttackTime` (`KismetSystemLibrary.GetGameTimeInSeconds`))
          (`KismetSystemLibrary.Delay` 0.2)
          (bind _returnvalue_3 (`|SpawnActorFromClass` "/Game/Characters/BadMoth/BP_MothProjectile.BP_MothProjectile_C" (`KismetMathLibrary.MakeTransform` _returnvalue_2 (`KismetMathLibrary.FindLookAtRotation` _returnvalue_2 (`self.K2_GetActorLocation` (`self.Player Ref`)))) "Undefined" "MultiplyWithRoot" null null))
          (`AudioComponent.Play` (`self.AttackAudio`) 0.0)
          (set `/Game/Characters/BadMoth/BP_MothProjectile.Damage` (`self.DamageDealt`) _returnvalue_3))))))

(event `self.BPC_dmgSys.onDeath`
  (bind _returnvalue (`self.K2_GetActorLocation`))
  (`KismetSystemLibrary.DelayUntilNextTick`)
  (`NiagaraFunctionLibrary.SpawnSystemAtLocation` "/Game/Characters/Enemy/NS_EnemyDeath.NS_EnemyDeath" _returnvalue)
  (for _ (range 7)
    (bind _returnvalue_2 (`|SpawnActorFromClass` "/Game/Spells/BP_ManaDroplet.BP_ManaDroplet_C" (`KismetMathLibrary.Conv_VectorToTransform` _returnvalue) "AlwaysSpawn" "MultiplyWithRoot" null null))
    (`/Engine/EditorBlueprintResources/StandardMacros.IsValid` _returnvalue_2
      (:`Is Valid`
        (`PrimitiveComponent.AddImpulse` (`/Game/Spells/BP_ManaDroplet.Sphere` _returnvalue_2) (* (`KismetMathLibrary.RandomUnitVector`) 5.0) "None" false))))
  (`self.K2_DestroyActor`))

(fn `doReceiveDamage`
  (params (dmgAmount :type "Float (double-precision)") (dmgResponse :type "/Game/HPSystem/dmgResponse Enum" :default "NewEnumerator0") (dmgType :type "/Game/HPSystem/dmgType Enum" :default "NewEnumerator0") (responseDuration :type "Float (double-precision)"))
  (returns (wasDamaged :type Boolean))
  (bind _skeletalmesh (`self.SkeletalMesh`))
  (`self.PlayHurtSound`)
  (bind _wasdamaged (`/Game/HPSystem/BPC_dmgSys.takeDamage` (`self.BPC_dmgSys`) dmgAmount dmgResponse dmgType responseDuration))
  (bind _returnvalue (`|SpawnActorFromClass` "/Game/Characters/Enemy/BP_DamageNumber.BP_DamageNumber_C" (`SceneComponent.K2_GetComponentToWorld` (`self.ExclamationMark`)) "Undefined" "MultiplyWithRoot" null null))
  (bind _aswbp_damage_number (cast `/Game/Characters/Enemy/WBP_DamageNumber` (`WidgetComponent.GetWidget` (`/Game/Characters/Enemy/BP_DamageNumber.Number` _returnvalue))))
  (set `/Game/Characters/Enemy/WBP_DamageNumber.Damage` dmgAmount _aswbp_damage_number)
  (if (> (- (`KismetSystemLibrary.GetGameTimeInSeconds`) (`self.lastDamageTakeTime`)) 0.2)
    (set `self.lastDamageTakeTime` (`KismetSystemLibrary.GetGameTimeInSeconds`))
    (for _index (range (`PrimitiveComponent.GetNumMaterials` _skeletalmesh))
      (`PrimitiveComponent.SetMaterial` _skeletalmesh _index (`self.FlashMat`))))
  (return _wasdamaged))

(fn `UserConstructionScript`)