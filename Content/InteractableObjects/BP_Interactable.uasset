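; BP_Interactable is an interactable object with a TextRender hover label and an empty Interact function.
; BeginPlay caches the label's authored text as HoverText, then blanks it.
; EnableText restores the cached text and DisableText clears it, while Tick keeps clearing it every frame that IsInteractable is false.
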(event `self.ReceiveBeginPlay`
  (set `self.hoverText` (`TextRenderComponent.Text` (`self.TextRender`)))
  (`self.DisableText`))

(event `self.ReceiveTick`
  (params (DeltaSeconds :type "Float (single-precision)"))
  (if (not (`self.isInteractable`))
    (`self.DisableText`)))

(fn `DisableText`
  (`TextRenderComponent.K2_SetText` (`self.TextRender`) ""))

(fn `EnableText`
  (`TextRenderComponent.K2_SetText` (`self.TextRender`) (`self.hoverText`)))

(fn `Interact`)

(fn `UserConstructionScript`)