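; Door Blueprint that stays locked unless the player holds a required item.
; IsLocked casts the player character to BP_ThirdPersonCharacter and reports unlocked when HasItem finds ItemToHave.
; Tick calls Interact every frame before running the parent's Tick.
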(event `self.ReceiveTick`
  (params (DeltaSeconds :type "Float (single-precision)"))
  (`self.Interact`)
  (`parent.ReceiveTick` DeltaSeconds))

(fn `isLocked`
  (returns (`locked?` :type Boolean))
  (bind _asbp_third_person_character (cast `/Game/ThirdPerson/Blueprints/BP_ThirdPersonCharacter` (`GameplayStatics.GetPlayerCharacter` 0)))
  (bind _has (`/Game/ThirdPerson/Blueprints/BP_ThirdPersonCharacter.HasItem` _asbp_third_person_character (`self.ItemToHave`)))
  (if _has
    (return false)
    (else
      (return true))))

(fn `UserConstructionScript`
  (`parent.UserConstructionScript`))