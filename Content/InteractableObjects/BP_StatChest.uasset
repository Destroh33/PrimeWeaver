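; Stat upgrade chest with a spinning book that offers the player a one-time choice of three random stat upgrades when interacted with.
; ChooseRandomUpgrade picks rows from DT_StatUpgrades, optionally unique.
; Interact shows them in WBP_UpgradeSelect and passes them, the widget and rolled percentages to the character's SelectUpgrade.
; Displayed and passed percentages are rolled separately, so they can differ.
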(event `self.ReceiveBeginPlay`
  (`parent.ReceiveBeginPlay`))

(event `self.ReceiveTick`
  (params (DeltaSeconds :type "Float (single-precision)"))
  (`SceneComponent.K2_AddRelativeRotation` (`self.book`) (`KismetMathLibrary.MakeRotator` 0.0 0.0 (* DeltaSeconds 45.0)) false false)
  (`parent.ReceiveTick` DeltaSeconds))

(fn `ChooseRandomUpgrade`
  (returns (Upgrades :type "Array of /Game/ThirdPerson/Blueprints/ST_StatUpgrade Structure"))
  (locals (RandomIndices :type "Array of Integer") (NewLocalVar :type "Array of Integer"))
  (bind _randomindices (`local.RandomIndices`))
  (bind _randomindices_2 (`local.RandomIndices`))
  (bind _random_upgrades (`self.Random Upgrades`))
  (bind _returnvalue (`KismetMathLibrary.RandomIntegerInRange` (`self.FirstIndex`) (`self.LastIndex`)))
  (while (< (`KismetArrayLibrary.Array_Length` _randomindices) (`self.NumChoices`))
    (if (`self.uniqueSpells`)
      (`KismetArrayLibrary.Array_AddUnique` _randomindices_2 _returnvalue)
      (else
        (`KismetArrayLibrary.Array_Add` _randomindices_2 _returnvalue))))
  (bind _outrownames (`DataTableFunctionLibrary.GetDataTableRowNames` "/Game/ThirdPerson/Blueprints/DT_StatUpgrades.DT_StatUpgrades"))
  (for _array_element _randomindices
    (bind _returnvalue_2 (`|GetDataTableRow` "/Game/ThirdPerson/Blueprints/DT_StatUpgrades.DT_StatUpgrades" (`|GetArrayItem` _outrownames _array_element))
      (:`then`
        (`KismetArrayLibrary.Array_Add` (`self.Random Upgrades`) _returnvalue_2))))
  (for _array_element_2 _random_upgrades
    (`KismetSystemLibrary.PrintText` (`|GenericToText` (`.StatType_3_5E4CDE31122A4DA297460D134909F74C` (break `/Game/ThirdPerson/Blueprints/ST_StatUpgrade` _array_element_2))) true true (struct :`G` 0.66 :`B` 1.0 :`A` 1.0) 5.0))
  (return _random_upgrades))

(fn `Interact`
  (bind _values (`self.Values`))
  (`parent.Interact`)
  (if (not (`self.used`))
    (set `self.used` true)
    (bind _upgrades (`self.ChooseRandomUpgrade`))
    (bind _output_get (set `self.Random Upgrades` _upgrades))
    (bind _returnvalue (`|CreateWidget` "/Game/InteractableObjects/WBP_UpgradeSelect.WBP_UpgradeSelect_C" (`GameplayStatics.GetPlayerController` 0)))
    (`UserWidget.AddToViewport` _returnvalue 0)
    (bind (_stattype _min _max) (break `/Game/ThirdPerson/Blueprints/ST_StatUpgrade` (`|GetArrayItem` _output_get)))
    (`TextBlock.SetText` (`/Game/InteractableObjects/WBP_UpgradeSelect.SpellName1` _returnvalue) (`KismetTextLibrary.Conv_StringToText` (`|GetEnumeratorNameAsString` _stattype)))
    (bind (_stattype_2 _min_2 _max_2) (break `/Game/ThirdPerson/Blueprints/ST_StatUpgrade` (`|GetArrayItem` _output_get 1)))
    (`TextBlock.SetText` (`/Game/InteractableObjects/WBP_UpgradeSelect.SpellName2` _returnvalue) (`KismetTextLibrary.Conv_StringToText` (`|GetEnumeratorNameAsString` _stattype_2)))
    (bind (_stattype_3 _min_3 _max_3) (break `/Game/ThirdPerson/Blueprints/ST_StatUpgrade` (`|GetArrayItem` _output_get 2)))
    (`TextBlock.SetText` (`/Game/InteractableObjects/WBP_UpgradeSelect.SpellName3` _returnvalue) (`KismetTextLibrary.Conv_StringToText` (`|GetEnumeratorNameAsString` _stattype_3)))
    (bind _returnvalue_2 (`KismetMathLibrary.Round` (`KismetMathLibrary.RandomFloatInRange` _min _max)))
    (`TextBlock.SetText` (`/Game/InteractableObjects/WBP_UpgradeSelect.ManaCost1` _returnvalue) (`KismetTextLibrary.Conv_StringToText` (`KismetStringLibrary.Concat_StrStr` "Increase by (in %): " (`KismetStringLibrary.Conv_IntToString` _returnvalue_2))))
    (bind _returnvalue_3 (`KismetMathLibrary.Round` (`KismetMathLibrary.RandomFloatInRange` _min_2 _max_2)))
    (`TextBlock.SetText` (`/Game/InteractableObjects/WBP_UpgradeSelect.ManaCost2` _returnvalue) (`KismetTextLibrary.Conv_StringToText` (`KismetStringLibrary.Concat_StrStr` "Increase by (in %): " (`KismetStringLibrary.Conv_IntToString` _returnvalue_3))))
    (bind _returnvalue_4 (`KismetMathLibrary.Round` (`KismetMathLibrary.RandomFloatInRange` _min_3 _max_3)))
    (`TextBlock.SetText` (`/Game/InteractableObjects/WBP_UpgradeSelect.ManaCost3` _returnvalue) (`KismetTextLibrary.Conv_StringToText` (`KismetStringLibrary.Concat_StrStr` "Increase by (in %): " (`KismetStringLibrary.Conv_IntToString` _returnvalue_4))))
    (`KismetArrayLibrary.Array_Add` _values _returnvalue_2)
    (`KismetArrayLibrary.Array_Add` _values _returnvalue_3)
    (`KismetArrayLibrary.Array_Add` _values _returnvalue_4)
    (bind _asbp_third_person_character (cast `/Game/ThirdPerson/Blueprints/BP_ThirdPersonCharacter` (`GameplayStatics.GetPlayerCharacter` 0)))
    (`/Game/ThirdPerson/Blueprints/BP_ThirdPersonCharacter.SelectUpgrade` _asbp_third_person_character (`self.Random Upgrades`) _returnvalue (`self.Values`))))

(fn `SetIcons`
  (params (Box :type "PanelWidget Object Reference") (SpellStruct :type "/Game/Spells/ST_WeaveCombo Structure"))
  (bind (_element1 _element2 _element3 _element4) (break `/Game/Spells/ST_WeaveCombo` SpellStruct))
  (for (_array_element _array_index) (`PanelWidget.GetAllChildren` Box)
    (bind _asimage (cast `Image` _array_element))
    (switch `/Game/Spells/Enum_ElementType` (select `int` _array_index :`0` _element1 :`1` _element2 :`2` _element3 :`3` _element4)
      (:`NewEnumerator0`
        (`Widget.SetVisibility` _asimage "Collapsed"))
      (:`NewEnumerator1`
        (`Image.SetBrush` _asimage (`WidgetBlueprintLibrary.MakeBrushFromTexture` "/Game/UI/fireicon.fireicon" 128 128)))
      (:`NewEnumerator2`
        (`Image.SetBrush` _asimage (`WidgetBlueprintLibrary.MakeBrushFromTexture` "/Game/UI/airicon.airicon" 128 128)))
      (:`NewEnumerator3`
        (`Image.SetBrush` _asimage (`WidgetBlueprintLibrary.MakeBrushFromTexture` "/Game/UI/rockicon.rockicon" 128 128)))
      (:`NewEnumerator4`
        (`Image.SetBrush` _asimage (`WidgetBlueprintLibrary.MakeBrushFromTexture` "/Game/UI/watericon.watericon" 128 128))))))

(fn `UserConstructionScript`
  (`parent.UserConstructionScript`))