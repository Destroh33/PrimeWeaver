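; BP_LockedDoor is an interactable door that sinks 1000 units below its starting position once opened.
; Interact calls OpenDoor and the parent Interact only if IsLocked returns false, which it always does here.
; OpenDoor sets the Move flag, and Tick then lerps the actor toward the target stored at BeginPlay, using DeltaSeconds as alpha for an eased descent.
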(event `self.ReceiveBeginPlay`
  (set `self.moveToLoc` (`KismetMathLibrary.MakeVector` (.x (`self.K2_GetActorLocation`)) (.y (`self.K2_GetActorLocation`)) (- (.z (`self.K2_GetActorLocation`)) 1000.0)))
  (`parent.ReceiveBeginPlay`))

(event `self.ReceiveTick`
  (params (DeltaSeconds :type "Float (single-precision)"))
  (if (`self.move`)
    (`self.K2_SetActorLocation` (`KismetMathLibrary.VLerp` (`self.K2_GetActorLocation`) (`self.moveToLoc`) DeltaSeconds))
    (`parent.ReceiveTick` DeltaSeconds)))

(fn `Interact`
  (bind _locked_ (`self.isLocked`))
  (if (not _locked_)
    (`self.OpenDoor`)
    (`parent.Interact`)))

(fn `isLocked`
  (returns (`locked?` :type Boolean))
  (return false))

(fn `OpenDoor`
  (set `self.move` true))

(fn `UserConstructionScript`
  (`parent.UserConstructionScript`))