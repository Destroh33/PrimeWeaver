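; Gust spell actor in Tier1Spells that throws its player straight up into the air.
; After a brief delay on BeginPlay, it checks that the player reference is valid and not falling, then launches the character with an overridden vertical velocity.
; A gust Niagara effect spawns attached to the player's mesh.
; The player reference arrives through SetPlayer, which also calls the parent version.
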(event `self.ReceiveBeginPlay`
  (bind _player_ref (`self.Player Ref`))
  (`KismetSystemLibrary.Delay` 0.01)
  (bind _ascharacter_movement_component (cast `CharacterMovementComponent` (`Pawn.GetMovementComponent` _player_ref)))
  (if (and (`KismetSystemLibrary.IsValid` _player_ref) (not (`NavMovementInterface.IsFalling` _ascharacter_movement_component)))
    (`Character.LaunchCharacter` _player_ref (0.0 0.0 1200.0) false true)
    (bind _returnvalue (`NiagaraFunctionLibrary.SpawnSystemAttached` "/Game/Spells/Tier1Spells/Gust/NE_Gust.NE_Gust" (`Character.Mesh` (`self.Player Ref`)) "None" (0.0 0.0 0.0) (struct) "KeepRelativeOffset"))
    (`PrimitiveComponent.SetPhysicsLinearVelocity` _returnvalue (0.0 0.0 0.0) false "None")
    (set `self.Niagara` null)))

(fn `SetPlayer`
  (params (PlayerRef :type "/Game/ThirdPerson/Blueprints/BP_ThirdPersonCharacter Object Reference"))
  (`parent.SetPlayer` PlayerRef)
  (set `self.Player Ref` PlayerRef))

(fn `UserConstructionScript`)