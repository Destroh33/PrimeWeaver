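; Tier 1 Ridge spell actor that rises out of the surface it targets, then sinks back and destroys itself.
; On BeginPlay a forward line trace, with a downward fallback from its end point, picks the target; if both miss, the actor is destroyed.
; It starts below the hit with only yaw kept.
; Tick lerps it up, then back down once a short lifetime since placement has passed.
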(event `self.ReceiveBeginPlay`
  (bind _returnvalue (`self.K2_GetActorLocation`))
  (bind _returnvalue_2 (+ _returnvalue (* (`self.GetActorForwardVector`) (1000.0 1000.0 1000.0))))
  (bind (_outhit _returnvalue_3) (`KismetSystemLibrary.LineTraceSingle` :`Start` _returnvalue :`End` _returnvalue_2 :`TraceChannel` "TraceTypeQuery1" :`DrawDebugType` "ForDuration"))
  (if _returnvalue_3
    (bind _output_get (set `self.TargetLocation` (`.Location` (`GameplayStatics.BreakHitResult` _outhit))))
    (bind _output_get_2 (set `self.StartLocation` (`KismetMathLibrary.MakeVector` (.x _output_get) (.y _output_get) (- (.z _output_get) 150.0))))
    (`self.K2_SetActorLocation` _output_get_2)
    (`self.K2_SetActorRotation` (`KismetMathLibrary.MakeRotator` 0.0 0.0 (.yaw (`self.K2_GetActorRotation`))))
    (set `self.StartTime` (`KismetSystemLibrary.GetGameTimeInSeconds`))
    (else
      (bind (_outhit_2 _returnvalue_4) (`KismetSystemLibrary.LineTraceSingle` :`Start` _returnvalue_2 :`End` (- _returnvalue_2 (0.0 0.0 2000.0)) :`TraceChannel` "TraceTypeQuery1" :`DrawDebugType` "ForDuration"))
      (if _returnvalue_4
        (bind _output_get_3 (set `self.TargetLocation` (`.Location` (`GameplayStatics.BreakHitResult` _outhit_2))))
        (bind _output_get_4 (set `self.StartLocation` (`KismetMathLibrary.MakeVector` (.x _output_get_3) (.y _output_get_3) (- (.z _output_get_3) 150.0))))
        (`self.K2_SetActorLocation` _output_get_4)
        (`self.K2_SetActorRotation` (`KismetMathLibrary.MakeRotator` 0.0 0.0 (.yaw (`self.K2_GetActorRotation`))))
        (set `self.StartTime` (`KismetSystemLibrary.GetGameTimeInSeconds`))
        (else
          (`KismetSystemLibrary.DelayUntilNextTick`)
          (`self.K2_DestroyActor`))))))

(event `self.ReceiveTick`
  (params (DeltaSeconds :type "Float (single-precision)"))
  (if (`self.isRising`)
    (bind _output_get (set `self.LerpAlpha` (`KismetMathLibrary.FClamp` (+ (`self.LerpAlpha`) (* (`self.RiseSpeed`) DeltaSeconds)))))
    (`self.K2_SetActorLocation` (`KismetMathLibrary.VLerp` (`self.StartLocation`) (`self.TargetLocation`) _output_get))
    (if (>= (`self.LerpAlpha`) 1.0)
      (set `self.isRising` false))
    (elif (and (> (- (`KismetSystemLibrary.GetGameTimeInSeconds`) (`self.StartTime`)) 2.0) (`self.isFalling`))
      (bind _output_get_2 (set `self.LerpAlphaDown` (`KismetMathLibrary.FClamp` (+ (`self.LerpAlphaDown`) (* (`self.RiseSpeed`) DeltaSeconds)))))
      (`self.K2_SetActorLocation` (`KismetMathLibrary.VLerp` (`self.TargetLocation`) (`self.StartLocation`) _output_get_2))
      (if (>= (`self.LerpAlphaDown`) 1.0)
        (set `self.isFalling` false))
      (elif (and (> (- (`KismetSystemLibrary.GetGameTimeInSeconds`) (`self.StartTime`)) 2.0) (not (`self.isFalling`)))
        (`self.K2_DestroyActor`)))))

(fn `UserConstructionScript`)