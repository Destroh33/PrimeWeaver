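; Elemental tornado spell actor that periodically damages nearby enemies and pulls them toward itself.
; Tick accumulates a timer that, every 0.3 seconds or so, triggers a box overlap query sized from the Hitbox component and filtered to BP_Enemy.
; Each enemy found receives fixed damage and a movement impulse toward the tornado's origin, scaled by that single frame's delta time.
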(event `self.ReceiveTick`
  (params (DeltaSeconds :type "Float (single-precision)"))
  (bind _hitbox (`self.Hitbox`))
  (`parent.ReceiveTick` DeltaSeconds)
  (bind _output_get (set `self.timer` (+ (`self.timer`) DeltaSeconds)))
  (if (> _output_get 0.3)
    (set `self.timer` 0.0)
    (`/Engine/EditorBlueprintResources/StandardMacros.IsValid` _hitbox
      (:`Is Valid`
        (bind _outactors (`KismetSystemLibrary.BoxOverlapActors` (`SceneComponent.K2_GetComponentLocation` _hitbox) (`BoxComponent.GetUnscaledBoxExtent` _hitbox) (`|MakeArray` "ObjectTypeQuery3" "ObjectTypeQuery2" :!type "EObjectTypeQuery Enum") "/Game/Characters/Enemy/BP_Enemy.BP_Enemy_C"))
        (for _array_element _outactors
          (bind _asbp_enemy (cast `/Game/Characters/Enemy/BP_Enemy` _array_element))
          (`/Game/Characters/Enemy/BP_Enemy.doReceiveDamage` _asbp_enemy 25.0 "NewEnumerator1" "NewEnumerator3" 0.0)
          (`CharacterMovementComponent.AddImpulse` (`Character.CharacterMovement` _asbp_enemy) (* (`KismetMathLibrary.NegateVector` (`KismetMathLibrary.Normal` (- (`self.K2_GetActorLocation` _asbp_enemy) (`self.K2_GetActorLocation`)))) (* DeltaSeconds 7500000.0)) false))))))

(fn `UserConstructionScript`
  (`parent.UserConstructionScript`))