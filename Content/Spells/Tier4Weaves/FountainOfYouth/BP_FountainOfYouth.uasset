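; Fountain of Youth tier 4 spell actor that, for a set duration, greatly boosts mana regeneration and changes mana and damage cooldowns.
; On BeginPlay it sets the rune count to 100, spends three runes, saves, zeroes the player's mana and attaches a Niagara well effect to the follow camera.
; A timer then fires Reset, which restores fixed values on the game instance, stops effect and audio, and destroys the actor.
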(event `reset`
  (set `/Game/Spells/WeaveGameInstance.ManaRegenPrime` 3.0 (stale `self.ReceiveBeginPlay` _asweave_game_instance))
  (set `/Game/Spells/WeaveGameInstance.ManaCooldown` 0.0 (stale `self.ReceiveBeginPlay` _asweave_game_instance))
  (set `/Game/Spells/WeaveGameInstance.DmgCooldown` 2.0 (stale `self.ReceiveBeginPlay` _asweave_game_instance))
  (bind _output_get (set `self.rain` (stale `self.ReceiveBeginPlay` _returnvalue)))
  (`ActorComponent.Deactivate` _output_get)
  (`AudioComponent.Stop` (`self.Audio`))
  (`self.K2_DestroyActor`))

(event `self.ReceiveBeginPlay`
  (bind _asbp_third_person_character (cast `/Game/ThirdPerson/Blueprints/BP_ThirdPersonCharacter` (`GameplayStatics.GetPlayerCharacter` 0)))
  (bind _asweave_game_instance (cast `/Game/Spells/WeaveGameInstance` (`GameplayStatics.GetGameInstance`)))
  (bind _saveref (`/Game/Spells/WeaveGameInstance.SaveRef` _asweave_game_instance))
  (set `/Game/Spells/WeaveSavedVals.RuneCount` 100 _saveref)
  (set `/Game/ThirdPerson/Blueprints/BP_ThirdPersonCharacter.CurrentSpellName` "None" _asbp_third_person_character)
  (bind _runecount (`/Game/Spells/WeaveSavedVals.RuneCount` _saveref))
  (if (>= _runecount 3)
    (bind _returnvalue (`NiagaraFunctionLibrary.SpawnSystemAttached` "/Game/Spells/Tier4Weaves/FountainOfYouth/NE_Well.NE_Well" (`MyProjectCharacter.FollowCamera` _asbp_third_person_character) "None" (0.0 0.0 0.0) (struct) "SnapToTargetIncludingScale"))
    (set `/Game/Spells/WeaveGameInstance.ManaCooldown` 2.0 _asweave_game_instance)
    (set `/Game/Spells/WeaveGameInstance.DmgCooldown` 0.0 _asweave_game_instance)
    (set `/Game/ThirdPerson/Blueprints/BP_ThirdPersonCharacter.CurrentMana` 0.0 _asbp_third_person_character)
    (set `/Game/Spells/WeaveGameInstance.ManaRegenPrime` 50.0 _asweave_game_instance)
    (set `self.YouthTimer` (`self.EffectDuration`))
    (bind _output_get (set `/Game/Spells/WeaveSavedVals.RuneCount` (- _runecount 3) _saveref))
    (`KismetSystemLibrary.PrintString` (`KismetStringLibrary.Conv_IntToString` _output_get))
    (`GameplayStatics.SaveGameToSlot` _saveref "WeaveSave")
    (`KismetSystemLibrary.K2_SetTimerDelegate` (delegate `reset`) (`self.EffectDuration`))))

(fn `SetPlayer`
  (params (PlayerRef :type "/Game/ThirdPerson/Blueprints/BP_ThirdPersonCharacter Object Reference"))
  (bind _output_get (set `self.Character` PlayerRef))
  (`parent.SetPlayer` _output_get))

(fn `UserConstructionScript`)