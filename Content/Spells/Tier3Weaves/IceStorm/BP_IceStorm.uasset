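; Ice Storm spell actor, a tier 3 weave that fires a spread of four BP_IceSpike actors.
; On BeginPlay it spawns all four at its own location and scale, each nudged a few random degrees right, left, down or up from its facing.
; It sets the same fixed damage on every spike and has no further logic of its own, not even destroying itself.
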(event `self.ReceiveBeginPlay`
  (bind _returnvalue (`self.GetTransform`))
  (bind _returnvalue_2 (`|SpawnActorFromClass` "/Game/Spells/Tier2Weaves/IceSpike/BP_IceSpike.BP_IceSpike_C" (`KismetMathLibrary.MakeTransform` (.location _returnvalue) (`KismetMathLibrary.MakeRotator` (.roll (.rotation _returnvalue)) (.pitch (.rotation _returnvalue)) (+ (.yaw (.rotation _returnvalue)) (`KismetMathLibrary.RandomFloatInRange` 1.0 3.0))) (.scale _returnvalue)) "Undefined" "MultiplyWithRoot" null null))
  (set `/Game/Spells/Tier2Weaves/IceSpike/BP_IceSpike.damage` 25.0 _returnvalue_2)
  (bind _returnvalue_3 (`|SpawnActorFromClass` "/Game/Spells/Tier2Weaves/IceSpike/BP_IceSpike.BP_IceSpike_C" (`KismetMathLibrary.MakeTransform` (.location _returnvalue) (`KismetMathLibrary.MakeRotator` (.roll (.rotation _returnvalue)) (.pitch (.rotation _returnvalue)) (+ (.yaw (.rotation _returnvalue)) (`KismetMathLibrary.RandomFloatInRange` -3.0 -1.0))) (.scale _returnvalue)) "Undefined" "MultiplyWithRoot" null null))
  (set `/Game/Spells/Tier2Weaves/IceSpike/BP_IceSpike.damage` 25.0 _returnvalue_3)
  (bind _returnvalue_4 (`|SpawnActorFromClass` "/Game/Spells/Tier2Weaves/IceSpike/BP_IceSpike.BP_IceSpike_C" (`KismetMathLibrary.MakeTransform` (.location _returnvalue) (`KismetMathLibrary.MakeRotator` (.roll (.rotation _returnvalue)) (+ (.pitch (.rotation _returnvalue)) (`KismetMathLibrary.RandomFloatInRange` -3.0 -1.0)) (.yaw (.rotation _returnvalue))) (.scale _returnvalue)) "Undefined" "MultiplyWithRoot" null null))
  (set `/Game/Spells/Tier2Weaves/IceSpike/BP_IceSpike.damage` 25.0 _returnvalue_4)
  (bind _returnvalue_5 (`|SpawnActorFromClass` "/Game/Spells/Tier2Weaves/IceSpike/BP_IceSpike.BP_IceSpike_C" (`KismetMathLibrary.MakeTransform` (.location _returnvalue) (`KismetMathLibrary.MakeRotator` (.roll (.rotation _returnvalue)) (+ (.pitch (.rotation _returnvalue)) (`KismetMathLibrary.RandomFloatInRange` 1.0 3.0)) (.yaw (.rotation _returnvalue))) (.scale _returnvalue)) "Undefined" "MultiplyWithRoot" null null))
  (set `/Game/Spells/Tier2Weaves/IceSpike/BP_IceSpike.damage` 25.0 _returnvalue_5))

(fn `UserConstructionScript`)