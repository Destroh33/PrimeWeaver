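; Fire Pillar spell actor, under Tier 3 Weaves, that deals fixed damage over time to enemies inside its Hitbox.
; An enemy entering the Hitbox takes damage at once and joins EnemyInRange, which a looping half-second timer damages until overlap ends.
; When a non-enemy overlaps, a box query at the sweep location finds enemies there, then damages and tracks them too.
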(event `DamageEnemyInRange`
  (for _array_element (`self.EnemyInRange`)
    (`/Game/Characters/Enemy/BP_Enemy.doReceiveDamage` _array_element 20.0 "NewEnumerator1" "NewEnumerator3" 0.0)))

(event `self.Hitbox.OnComponentBeginOverlap`
  (params (OverlappedComponent :type "PrimitiveComponent Object Reference") (OtherActor :type "Actor Object Reference") (OtherComp :type "PrimitiveComponent Object Reference") (OtherBodyIndex :type Integer) (bFromSweep :type Boolean) (SweepResult :type "HitResult Structure (by ref)"))
  (bind _asbp_enemy (cast `/Game/Characters/Enemy/BP_Enemy` OtherActor)
    (:`then`
      (`/Game/Characters/BadSpider/BP_BadSpida.doReceiveDamage` _asbp_enemy 20.0 "NewEnumerator1" "NewEnumerator3" 0.0)
      (`KismetArrayLibrary.Array_AddUnique` (`self.EnemyInRange`) _asbp_enemy))
    (:`CastFailed`
      (bind _outactors (`KismetSystemLibrary.BoxOverlapActors` (`.Location` (`GameplayStatics.BreakHitResult` SweepResult)) (`BoxComponent.GetUnscaledBoxExtent` (`self.Hitbox`)) (`|MakeArray` "ObjectTypeQuery2" :!type "EObjectTypeQuery Enum") "/Game/Characters/Enemy/BP_Enemy.BP_Enemy_C" (`|MakeArray` OtherActor)))
      (for _array_element _outactors
        (bind _asbp_enemy_2 (cast `/Game/Characters/Enemy/BP_Enemy` _array_element))
        (`/Game/Characters/BadSpider/BP_BadSpida.doReceiveDamage` _asbp_enemy_2 20.0 "NewEnumerator1" "NewEnumerator3" 0.0)
        (`KismetArrayLibrary.Array_AddUnique` (`self.EnemyInRange`) _asbp_enemy_2)))))

(event `self.ReceiveBeginPlay`
  (`parent.ReceiveBeginPlay`)
  (bind _returnvalue (`KismetSystemLibrary.K2_SetTimerDelegate` (delegate `DamageEnemyInRange`) 0.5 true)))

(event `self.Hitbox.OnComponentEndOverlap`
  (params (OverlappedComponent :type "PrimitiveComponent Object Reference") (OtherActor :type "Actor Object Reference") (OtherComp :type "PrimitiveComponent Object Reference") (OtherBodyIndex :type Integer))
  (bind _asbp_enemy (cast `/Game/Characters/Enemy/BP_Enemy` OtherActor))
  (`KismetArrayLibrary.Array_RemoveItem` (`self.EnemyInRange`) _asbp_enemy))

(fn `UserConstructionScript`
  (`parent.UserConstructionScript`))