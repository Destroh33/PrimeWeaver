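; BP_MoltenArmor is a Tier 3 weave spell actor that shields its owning player with retaliatory molten armor.
; On spawn it sends the DA_MoltenArmor effect to the player, then destroys itself after the effect's duration.
; Each tick it snaps to the player and checks for recently taken damage.
; A recent hit triggers a throttled radial impulse and damages every BP_Enemy overlapping its sphere.
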(event `self.ReceiveBeginPlay`
  (`parent.ReceiveBeginPlay`)
  (`KismetSystemLibrary.Delay` 0.1)
  (message `/Game/HPSystem/dmgSystem.doReceiveEffect` (`self.OwningPlayer`) "/Game/Spells/Tier3Weaves/MoltenArmor/DA_MoltenArmor.DA_MoltenArmor")
  (`KismetSystemLibrary.Delay` (`/Game/HPSystem/Effects/PDA_effectData.Duration` (`self.ArmorEffectObj`)))
  (`self.K2_DestroyActor`))

(event `self.ReceiveTick`
  (params (DeltaSeconds :type "Float (single-precision)"))
  (bind _returnvalue (`KismetSystemLibrary.GetGameTimeInSeconds`))
  (bind _owningplayer (`self.OwningPlayer`))
  (`parent.ReceiveTick` DeltaSeconds)
  (`SceneComponent.K2_SetWorldTransform` (`self.Scene`) (`self.GetTransform` _owningplayer) false true)
  (if (and (> (- _returnvalue (`self.LastImpulseTriggerTime`)) 0.2) (< (- _returnvalue (`/Game/ThirdPerson/Blueprints/BP_ThirdPersonCharacter.lastDamageTakeTime` _owningplayer)) 0.2))
    (`SceneComponent.K2_SetWorldLocation` (`self.RadialForce`) (`SceneComponent.K2_GetComponentLocation` (`Character.CapsuleComponent` _owningplayer)) false true)
    (`RadialForceComponent.FireImpulse` (`self.RadialForce`))
    (for _array_element (`PrimitiveComponent.GetOverlappingActors` (`self.Sphere`) "/Game/Characters/Enemy/BP_Enemy.BP_Enemy_C")
      (bind _asbp_enemy (cast `/Game/Characters/Enemy/BP_Enemy` _array_element))
      (`/Game/Characters/Enemy/BP_Enemy.doReceiveDamage` _asbp_enemy 10.0 "NewEnumerator2" "NewEnumerator3" 3.0))
    (set `self.LastImpulseTriggerTime` (`KismetSystemLibrary.GetGameTimeInSeconds`))))

(fn `UserConstructionScript`
  (`parent.UserConstructionScript`))