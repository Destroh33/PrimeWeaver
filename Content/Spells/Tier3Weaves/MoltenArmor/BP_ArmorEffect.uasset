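; BP_ArmorEffect is the Molten Armor spell effect that protects the target third-person character while active.
; On apply, it halves the character's damage multiplier, adds a molten overlay material keyed by effect class, and blocks negative effects.
; On expire, it resets the multiplier and requests overlay removal.
; It restores negative-effect susceptibility only if the damage system counts no more than one instance of this effect.
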(event `/Game/HPSystem/Effects/effectInterface.onApply`
  (params (EffectContext :type "/Game/HPSystem/Effects/S_effectContext Structure"))
  (bind _asbp_third_person_character (cast `/Game/ThirdPerson/Blueprints/BP_ThirdPersonCharacter` (`.To_22_DDB7CF14C7374795BF77CFBF72EBAC74` (break `/Game/HPSystem/Effects/S_effectContext` EffectContext))))
  (set `/Game/ThirdPerson/Blueprints/BP_ThirdPersonCharacter.DamageMultiplier` 0.5 _asbp_third_person_character)
  (`/Game/ThirdPerson/Blueprints/BP_ThirdPersonCharacter.doApplyOverlayMaterial` _asbp_third_person_character "/Game/Spells/Tier3Weaves/MoltenArmor/M_MoltenArmor.M_MoltenArmor" "BP_ArmorEffect_C")
  (set `/Game/ThirdPerson/Blueprints/BP_ThirdPersonCharacter.CanReceiveNegativeEffect` false _asbp_third_person_character))

(event `/Game/HPSystem/Effects/effectInterface.onExpire`
  (params (EffectContext :type "/Game/HPSystem/Effects/S_effectContext Structure"))
  (bind _asbp_third_person_character (cast `/Game/ThirdPerson/Blueprints/BP_ThirdPersonCharacter` (`.To_22_DDB7CF14C7374795BF77CFBF72EBAC74` (break `/Game/HPSystem/Effects/S_effectContext` EffectContext))))
  (set `/Game/ThirdPerson/Blueprints/BP_ThirdPersonCharacter.DamageMultiplier` 1.0 _asbp_third_person_character)
  (`/Game/HPSystem/dmgSystem.doRemoveOverlayMaterial` _asbp_third_person_character "BP_ArmorEffect_C")
  (bind _count (`/Game/HPSystem/BPC_dmgSys.getEffectClassCount` (`/Game/ThirdPerson/Blueprints/BP_ThirdPersonCharacter.BPC_dmgSys` _asbp_third_person_character) "BP_ArmorEffect_C"))
  (if (not (> _count 1))
    (set `/Game/ThirdPerson/Blueprints/BP_ThirdPersonCharacter.CanReceiveNegativeEffect` true _asbp_third_person_character)))