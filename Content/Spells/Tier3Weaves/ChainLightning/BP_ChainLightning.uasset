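; Chain lightning spell actor that fires a bolt on BeginPlay, damaging the first enemy its forward visibility trace hits.
; From that enemy, Chain recursively sphere-overlaps nearby BP_Enemy actors and damages each one.
; A HitActors list keeps any enemy from being struck twice.
; Each link spawns a Niagara lightning effect with start and end vector parameters, and only the first hit plays the electricity sound.
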(event `self.ReceiveBeginPlay`
  (bind _returnvalue (`self.K2_GetActorLocation`))
  (bind _returnvalue_2 (+ (* (`self.GetActorForwardVector`) (3000.0 3000.0 3000.0)) _returnvalue))
  (bind _returnvalue_3 (`NiagaraFunctionLibrary.SpawnSystemAtLocation` "/Game/Spells/Tier2Weaves/Lightning/LightningEffect.LightningEffect" _returnvalue))
  (`NiagaraComponent.SetVariableVec3` _returnvalue_3 "LightningStart" _returnvalue)
  (bind (_outhit _returnvalue_4) (`KismetSystemLibrary.LineTraceSingle` :`Start` _returnvalue :`End` _returnvalue_2 :`TraceChannel` "TraceTypeQuery1" :`DrawTime` 1.0))
  (if _returnvalue_4
    (bind (_bblockinghit _binitialoverlap _time _distance _location _impactpoint _normal _impactnormal _physmat _hitactor) (`GameplayStatics.BreakHitResult` _outhit))
    (`NiagaraComponent.SetVariableVec3` _returnvalue_3 "LightningEnd" _location)
    (bind _asbp_enemy (cast `/Game/Characters/Enemy/BP_Enemy` _hitactor))
    (`/Game/Characters/Enemy/BP_Enemy.doReceiveDamage` _asbp_enemy 60.0 "NewEnumerator1" "NewEnumerator2" 0.0)
    (bind _returnvalue_5 (`self.K2_GetActorLocation` _asbp_enemy))
    (`GameplayStatics.PlaySoundAtLocation` "/Game/Sounds/electriciy_Cue.electriciy_Cue" _returnvalue_5 (struct) 1.0 1.0 0.0 null null null null)
    (`KismetArrayLibrary.Array_Add` (`self.HitActors`) _asbp_enemy)
    (`self.Chain` _returnvalue_5)
    (else
      (`NiagaraComponent.SetVariableVec3` _returnvalue_3 "LightningEnd" _returnvalue_2))))

(fn `Chain`
  (params (StartLoc :type "Vector Structure"))
  (bind _outactors (`KismetSystemLibrary.SphereOverlapActors` StartLoc 250.0 (`|MakeArray` "ObjectTypeQuery2" :!type "EObjectTypeQuery Enum") "/Game/Characters/Enemy/BP_Enemy.BP_Enemy_C" (`self.HitActors`)))
  (for _array_element _outactors
    (bind _asbp_enemy (cast `/Game/Characters/Enemy/BP_Enemy` _array_element))
    (if (not (`KismetArrayLibrary.Array_Contains` (`self.HitActors`) _asbp_enemy))
      (bind _returnvalue (`NiagaraFunctionLibrary.SpawnSystemAtLocation` "/Game/Spells/Tier2Weaves/Lightning/LightningEffect.LightningEffect" StartLoc))
      (`NiagaraComponent.SetVariableVec3` _returnvalue "LightningStart" StartLoc)
      (bind _returnvalue_2 (`self.K2_GetActorLocation` _asbp_enemy))
      (`NiagaraComponent.SetVariableVec3` _returnvalue "LightningEnd" _returnvalue_2)
      (`/Game/Characters/Enemy/BP_Enemy.doReceiveDamage` _asbp_enemy 60.0 "NewEnumerator1" "NewEnumerator2" 0.0)
      (`KismetArrayLibrary.Array_Add` (`self.HitActors`) _asbp_enemy)
      (`self.Chain` _returnvalue_2))))

(fn `UserConstructionScript`)