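; BP_LavaBomb is a lava bomb spell projectile that explodes on impact, damaging nearby enemies.
; On spawn, its collision sphere drives the projectile movement but stays non-colliding until a launch delay passes.
; On hit, it moves the radial force slightly below the impact point and uses that component's radius to find and damage BP_Enemy actors.
; It then fires the physics impulse and destroys itself.
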(event `self.ReceiveBeginPlay`
  (bind _sphere (`self.Sphere`))
  (`MovementComponent.SetUpdatedComponent` (`self.ProjectileMovement`) (`self.Sphere`))
  (`PrimitiveComponent.SetCollisionEnabled` _sphere "NoCollision")
  (`KismetSystemLibrary.Delay` (`self.LaunchDelay`))
  (`PrimitiveComponent.SetCollisionEnabled` _sphere "QueryAndPhysics"))

(event `self.Sphere.OnComponentHit`
  (params (HitComponent :type "PrimitiveComponent Object Reference") (OtherActor :type "Actor Object Reference") (OtherComp :type "PrimitiveComponent Object Reference") (NormalImpulse :type "Vector Structure") (Hit :type "HitResult Structure (by ref)"))
  (bind _explosionforce (`self.ExplosionForce`))
  (`SceneComponent.K2_SetWorldLocation` _explosionforce (+ (`.Location` (`GameplayStatics.BreakHitResult` Hit)) (0.0 0.0 -32.0)) false true)
  (bind _outactors (`KismetSystemLibrary.SphereOverlapActors` (`SceneComponent.K2_GetComponentLocation` _explosionforce) (`RadialForceComponent.Radius` _explosionforce) (`|MakeArray` "ObjectTypeQuery2" :!type "EObjectTypeQuery Enum") "/Game/Characters/Enemy/BP_Enemy.BP_Enemy_C"))
  (for _array_element _outactors
    (bind _asbp_enemy (cast `/Game/Characters/Enemy/BP_Enemy` _array_element))
    (`/Game/Characters/Enemy/BP_Enemy.doReceiveDamage` _asbp_enemy (`self.BaseDamage`) "NewEnumerator1" "NewEnumerator2" 0.0))
  (`RadialForceComponent.FireImpulse` (`self.ExplosionForce`))
  (`self.K2_DestroyActor`))

(fn `UserConstructionScript`
  (`parent.UserConstructionScript`))