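; BP_IceSpike is an ice spike spell projectile that spins as it flies and damages enemies it passes through.
; Projectile movement drives a collision sphere, while Tick spins the mesh.
; Overlaps damage BP_Enemy actors until a blocking hit stops the spin and Niagara effect, plays an impact sound and disables further damage.
; That hit, or overlapping anything other than enemies and fellow spikes, destroys the spike after a short delay.
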(event `self.Sphere.OnComponentBeginOverlap`
  (params (OverlappedComponent :type "PrimitiveComponent Object Reference") (OtherActor :type "Actor Object Reference") (OtherComp :type "PrimitiveComponent Object Reference") (OtherBodyIndex :type Integer) (bFromSweep :type Boolean) (SweepResult :type "HitResult Structure (by ref)"))
  (cast `/Game/Spells/Tier2Weaves/IceSpike/BP_IceSpike` OtherActor
    (:`CastFailed`
      (bind _asbp_enemy (cast `/Game/Characters/Enemy/BP_Enemy` OtherActor)
        (:`then`
          (if (not (`self.hitNonEnemy`))
            (`/Game/Characters/BadSpider/BP_BadSpida.doReceiveDamage` _asbp_enemy (`self.damage`) "NewEnumerator1" "NewEnumerator2" 0.0)))
        (:`CastFailed`
          (`KismetSystemLibrary.Delay` 2.0 :!label _label)
          (`self.K2_DestroyActor`))))))

(event `self.ReceiveBeginPlay`
  (`MovementComponent.SetUpdatedComponent` (`self.ProjectileMovement`) (`self.Sphere`)))

(event `self.ReceiveTick`
  (params (DeltaSeconds :type "Float (single-precision)"))
  (if (`self.spinning`)
    (`SceneComponent.K2_AddLocalRotation` (`self.IceSpikeMesh`) (`KismetMathLibrary.MakeRotator` 0.0 0.0 (* DeltaSeconds 1080.0)) false false)))

(event `self.Sphere.OnComponentHit`
  (params (HitComponent :type "PrimitiveComponent Object Reference") (OtherActor :type "Actor Object Reference") (OtherComp :type "PrimitiveComponent Object Reference") (NormalImpulse :type "Vector Structure") (Hit :type "HitResult Structure (by ref)"))
  (set `self.hitNonEnemy` true)
  (`ActorComponent.Deactivate` (`self.Niagara`))
  (set `self.spinning` false)
  (`GameplayStatics.PlaySoundAtLocation` "/Game/Sounds/pound_sharp_Cue.pound_sharp_Cue" (`SceneComponent.K2_GetComponentLocation` (`self.Sphere`)) (struct) 1.0 1.0 0.15 null null null null)
  (goto _label))

(fn `UserConstructionScript`)