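; Meteor Slam spell actor that drives an airborne player into the ground to damage nearby enemies, destroying itself if the player is not falling.
; On BeginPlay it records the starting height and launches the player downward.
; Tick detects the landing once, plays sound and Niagara effects, then sphere-overlaps for enemies.
; Damage, response duration and upward knock-up all scale with the height fallen.
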(event `self.ReceiveBeginPlay`
  (bind _player_ref (`self.Player Ref`))
  (`KismetSystemLibrary.DelayUntilNextTick`)
  (if (`NavMovementComponent.IsFalling` (`Character.CharacterMovement` _player_ref))
    (set `self.InitialZ` (.z (`self.K2_GetActorLocation` _player_ref)))
    (`Character.LaunchCharacter` _player_ref (0.0 0.0 -2500.0) false true)
    (else
      (`self.K2_DestroyActor`))))

(event `self.ReceiveTick`
  (params (DeltaSeconds :type "Float (single-precision)"))
  (bind _player_ref (`self.Player Ref`))
  (bind _returnvalue (`self.K2_GetActorLocation` _player_ref))
  (`KismetSystemLibrary.DelayUntilNextTick`)
  (if (and (not (`NavMovementComponent.IsFalling` (`Character.CharacterMovement` _player_ref))) (not (`self.slammed`)))
    (set `self.slammed` true)
    (bind _output_get (set `self.FinalZ` (.z _returnvalue)))
    (`GameplayStatics.PlaySound2D` "/Game/Sounds/rock_crash_Cue.rock_crash_Cue" 1.0 1.0 0.0 null null)
    (`NiagaraFunctionLibrary.SpawnSystemAtLocation` "/Game/Spells/Tier2Weaves/MeteorSlam/NS_MeteorSlam.NS_MeteorSlam" (`self.K2_GetActorLocation` (`self.Player Ref`)))
    (bind _outactors (`KismetSystemLibrary.SphereOverlapActors` _returnvalue 500.0 (`|MakeArray` "ObjectTypeQuery2" "ObjectTypeQuery3" :!type "EObjectTypeQuery Enum") "/Game/Characters/Enemy/BP_Enemy.BP_Enemy_C"))
    (for _array_element _outactors
      (bind _asbp_enemy (cast `/Game/Characters/Enemy/BP_Enemy` _array_element))
      (bind _returnvalue_2 (- (`self.InitialZ`) _output_get))
      (bind _returnvalue_3 (* _returnvalue_2 0.065))
      (`/Game/HPSystem/dmgSystem.doReceiveDamage` _asbp_enemy _returnvalue_3 "NewEnumerator2" "NewEnumerator1" (* _returnvalue_3 0.05))
      (`Character.LaunchCharacter` _asbp_enemy (`KismetMathLibrary.MakeVector` 0.0 0.0 _returnvalue_2) false true))))

(fn `SetPlayer`
  (params (PlayerRef :type "/Game/ThirdPerson/Blueprints/BP_ThirdPersonCharacter Object Reference"))
  (bind _output_get (set `self.Player Ref` PlayerRef))
  (`parent.SetPlayer` _output_get))

(fn `UserConstructionScript`
  (`parent.UserConstructionScript`))