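; Chargeable fireball spell projectile that explodes on impact, damaging nearby BP_Enemy actors.
; While charging, it follows the owning player's launch transform, scaling collision size, Niagara charge effect, damage, and explosion radius and impulse with hold time.
; Releasing the charge launches it forward and upward, enabling collision after a short delay.
; On hit, it spawns charge-scaled explosion VFX, applies damage through a sphere overlap, fires a radial impulse and destroys itself.
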(event `/Game/Spells/BPI_ChargeableWeave.EndCharging`
  (bind _sphere (`self.Sphere`))
  (bind _projectilemovement (`self.ProjectileMovement`))
  (set `self.IsCharging` false)
  (`NiagaraComponent.SetVariableBool` (`self.NS_BigFireball`) "TrailEnabled" true)
  (bind _offsetedtransform (`self.GetOffsettedTransform`))
  (`self.K2_SetActorTransform` _offsetedtransform false true)
  (`ProjectileMovementComponent.SetVelocityInLocalSpace` _projectilemovement (* (`ProjectileMovementComponent.InitialSpeed` _projectilemovement) (1.0 0.0 0.5)))
  (`MovementComponent.SetUpdatedComponent` (`self.ProjectileMovement`) _sphere)
  (`ActorComponent.Activate` (`self.ProjectileMovement`) false)
  (`KismetSystemLibrary.Delay` (`self.LaunchDelay`))
  (`PrimitiveComponent.SetCollisionEnabled` _sphere "QueryAndPhysics"))

(event `/Game/Spells/BPI_ChargeableWeave.BeginCharging`
  (set `self.IsCharging` true)
  (`NiagaraComponent.SetVariableBool` (`self.NS_BigFireball`) "TrailEnabled" false))

(event `self.ReceiveBeginPlay`
  (bind _sphere (`self.Sphere`))
  (`PrimitiveComponent.SetCollisionEnabled` _sphere "NoCollision")
  (bind _returnvalue (`GameplayStatics.SpawnSoundAttached` "/Game/Sounds/blazing_fire_Cue.blazing_fire_Cue" _sphere "None" (0.0 0.0 0.0) (struct) "KeepRelativeOffset" false 1.0 1.0 0.0 null null))
  (set `self.fireSound` _returnvalue))

(event `self.Sphere.OnComponentHit`
  (params (HitComponent :type "PrimitiveComponent Object Reference") (OtherActor :type "Actor Object Reference") (OtherComp :type "PrimitiveComponent Object Reference") (NormalImpulse :type "Vector Structure") (Hit :type "HitResult Structure (by ref)"))
  (bind (_bblockinghit _binitialoverlap _time _distance _location) (`GameplayStatics.BreakHitResult` Hit))
  (bind _explosionforce (`self.ExplosionForce`))
  (bind _firesound (`self.fireSound`))
  (bind _basedamage (`self.BaseDamage`))
  (`AudioComponent.Stop` _firesound)
  (`ActorComponent.K2_DestroyComponent` _firesound)
  (`GameplayStatics.PlaySoundAtLocation` "/Game/Sounds/explosion_Cue.explosion_Cue" _location (struct) 1.0 1.0 0.0 null null null null)
  (bind _returnvalue (`NiagaraFunctionLibrary.SpawnSystemAtLocation` "/Game/Spells/Tier2Weaves/BigFireball/NE_BigFireballExplosionSystem.NE_BigFireballExplosionSystem" _location (struct) (1.0 1.0 1.0) true false))
  (`NiagaraComponent.SetVariableFloat` _returnvalue "ChargeLevel" (`self.ChargeLevel`))
  (`ActorComponent.Activate` _returnvalue false)
  (`SceneComponent.K2_SetWorldLocation` _explosionforce _location false true)
  (bind _outactors (`KismetSystemLibrary.SphereOverlapActors` (`SceneComponent.K2_GetComponentLocation` _explosionforce) (`RadialForceComponent.Radius` _explosionforce) (`|MakeArray` "ObjectTypeQuery2" :!type "EObjectTypeQuery Enum") "/Game/Characters/Enemy/BP_Enemy.BP_Enemy_C"))
  (for _array_element _outactors
    (bind _asbp_enemy (cast `/Game/Characters/Enemy/BP_Enemy` _array_element))
    (`/Game/Characters/Enemy/BP_Enemy.doReceiveDamage` _asbp_enemy _basedamage "NewEnumerator1" "NewEnumerator2" 0.0)
    (`KismetSystemLibrary.PrintString` (`KismetStringLibrary.Conv_DoubleToString` _basedamage)))
  (`RadialForceComponent.FireImpulse` (`self.ExplosionForce`))
  (`self.K2_DestroyActor`))

(event `self.ReceiveTick`
  (params (DeltaSeconds :type "Float (single-precision)"))
  (`parent.ReceiveTick` DeltaSeconds)
  (if (`self.IsCharging`)
    (set `self.ChargedTime` (+ DeltaSeconds (`self.ChargedTime`)))
    (`self.ChargeFireballProperties`)
    (bind _offsetedtransform (`self.GetOffsettedTransform`))
    (`self.K2_SetActorTransform` _offsetedtransform false true)
    (else
      (set `self.ChargedTime` 0.0))))

(fn `ChargeFireballProperties`
  (bind _explosionforce (`self.ExplosionForce`))
  (bind _returnvalue (`KismetMathLibrary.FMin` (/ (`self.ChargedTime`) (`self.MaxChargeTime`)) 1.0))
  (`SphereComponent.SetSphereRadius` (`self.Sphere`) (`KismetMathLibrary.Lerp` (`self.MinSize`) (`self.MaxSize`) _returnvalue) true)
  (`NiagaraComponent.SetVariableFloat` (`self.NS_BigFireball`) "ChargeLevel" (`|EaseFunction` "ExpoOut" _returnvalue 0.0 1.0))
  (set `RadialForceComponent.Radius` (`KismetMathLibrary.Lerp` (`self.minExplosionRadius`) (`self.maxExplosionRadius`) _returnvalue) _explosionforce)
  (set `RadialForceComponent.ImpulseStrength` (`KismetMathLibrary.Lerp` (`self.minExplosionImpulse`) (`self.maxExplosionImpulse`) _returnvalue) _explosionforce)
  (set `self.BaseDamage` (`KismetMathLibrary.Lerp` (`self.MinDamage`) (`self.MaxDamage`) _returnvalue))
  (set `self.ChargeLevel` _returnvalue))

(fn `GetOffsettedTransform`
  (returns (OffsetedTransform :type "Transform Structure"))
  (bind _transform (`/Game/ThirdPerson/Blueprints/BP_ThirdPersonCharacter.GetSpellLaunchTransform` (`self.OwningPlayer`)))
  (bind _rotation (.rotation _transform))
  (return (`KismetMathLibrary.MakeTransform` (+ (.location _transform) (* (`KismetMathLibrary.GetForwardVector` _rotation) (`self.MaxSize`))) _rotation (.scale _transform))))

(fn `UserConstructionScript`
  (`parent.UserConstructionScript`))