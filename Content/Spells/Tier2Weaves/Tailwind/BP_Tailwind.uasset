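; BP_Tailwind is a spell actor that grants its player a five-second boost to walk speed and jump velocity.
; On BeginPlay it waits a tick, raises both values to 1.5x the player's defaults, attaches a wind Niagara effect and plays a sound.
; Tick keeps reapplying the boost until the delay ends, when the defaults are restored and the actor destroys itself.
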(event `self.ReceiveBeginPlay`
  (bind _player_ref (`self.Player Ref`))
  (bind _defaultjumpvel (`/Game/ThirdPerson/Blueprints/BP_ThirdPersonCharacter.DefaultJumpVel` _player_ref))
  (bind _defaultwalkspeed (`/Game/ThirdPerson/Blueprints/BP_ThirdPersonCharacter.DefaultWalkSpeed` _player_ref))
  (`KismetSystemLibrary.DelayUntilNextTick`)
  (bind _ascharacter_movement_component (cast `CharacterMovementComponent` (`Pawn.GetMovementComponent` _player_ref)))
  (set `self.As Character Movement Component` _ascharacter_movement_component)
  (if (`KismetSystemLibrary.IsValid` _player_ref)
    (set `CharacterMovementComponent.JumpZVelocity` (* _defaultjumpvel 1.5) _ascharacter_movement_component)
    (set `CharacterMovementComponent.MaxWalkSpeed` (* _defaultwalkspeed 1.5) _ascharacter_movement_component)
    (`NiagaraFunctionLibrary.SpawnSystemAttached` "/Game/Spells/Tier2Weaves/Tailwind/NS_Tailwind.NS_Tailwind" (`Character.Mesh` (`self.Player Ref`)) "None" (0.0 0.0 40.0) (struct) "KeepRelativeOffset" true)
    (`AudioComponent.Play` (`self.wind_sfx`) 0.0)
    (`KismetSystemLibrary.Delay` 5.0)
    (set `CharacterMovementComponent.JumpZVelocity` _defaultjumpvel _ascharacter_movement_component)
    (set `CharacterMovementComponent.MaxWalkSpeed` _defaultwalkspeed _ascharacter_movement_component)
    (`self.K2_DestroyActor`)))

(event `self.ReceiveTick`
  (params (DeltaSeconds :type "Float (single-precision)"))
  (bind _player_ref (`self.Player Ref`))
  (bind _as_character_movement_component (`self.As Character Movement Component`))
  (`KismetSystemLibrary.DelayUntilNextTick`)
  (set `CharacterMovementComponent.JumpZVelocity` (* (`/Game/ThirdPerson/Blueprints/BP_ThirdPersonCharacter.DefaultJumpVel` _player_ref) 1.5) _as_character_movement_component)
  (set `CharacterMovementComponent.MaxWalkSpeed` (* (`/Game/ThirdPerson/Blueprints/BP_ThirdPersonCharacter.DefaultWalkSpeed` _player_ref) 1.5) _as_character_movement_component))

(fn `SetPlayer`
  (params (PlayerRef :type "/Game/ThirdPerson/Blueprints/BP_ThirdPersonCharacter Object Reference"))
  (`parent.SetPlayer` PlayerRef)
  (set `self.Player Ref` PlayerRef))

(fn `UserConstructionScript`)