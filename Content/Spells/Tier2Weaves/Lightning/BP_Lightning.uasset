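; BP_Lightning is a Tier 2 weave spell actor that fires an instant lightning bolt along its forward vector when spawned.
; On BeginPlay, a fixed-range Visibility line trace sets the lightning effect's end point to the impact, or to maximum range on a miss.
; If the trace hits a BP_Enemy, it applies fixed damage, sets the Hit flag and plays an electricity sound at the impact.
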(event `self.ReceiveBeginPlay`
  (bind _returnvalue (`self.K2_GetActorLocation`))
  (bind _lightningeffect (`self.LightningEffect`))
  (bind _returnvalue_2 (+ (* (`self.GetActorForwardVector`) (3000.0 3000.0 3000.0)) _returnvalue))
  (`NiagaraComponent.SetVariableVec3` _lightningeffect "LightningStart" _returnvalue)
  (bind (_outhit _returnvalue_3) (`KismetSystemLibrary.LineTraceSingle` :`Start` _returnvalue :`End` _returnvalue_2 :`TraceChannel` "TraceTypeQuery1" :`DrawTime` 1.0))
  (if _returnvalue_3
    (bind (_bblockinghit _binitialoverlap _time _distance _location _impactpoint _normal _impactnormal _physmat _hitactor) (`GameplayStatics.BreakHitResult` _outhit))
    (`NiagaraComponent.SetVariableVec3` _lightningeffect "LightningEnd" _location)
    (bind _asbp_enemy (cast `/Game/Characters/Enemy/BP_Enemy` _hitactor))
    (`/Game/Characters/Enemy/BP_Enemy.doReceiveDamage` _asbp_enemy 50.0 "NewEnumerator1" "NewEnumerator2" 0.0)
    (set `self.hit` true)
    (`GameplayStatics.PlaySoundAtLocation` "/Game/Sounds/electriciy_Cue.electriciy_Cue" _location (struct) 1.0 1.0 0.0 null null null null)
    (else
      (`NiagaraComponent.SetVariableVec3` _lightningeffect "LightningEnd" _returnvalue_2))))

(fn `UserConstructionScript`)