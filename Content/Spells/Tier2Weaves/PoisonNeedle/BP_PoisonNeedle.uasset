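; BP_PoisonNeedle is a Tier 2 Weave spell projectile that damages third-person characters it overlaps.
; Any overlap stops its ProjectileMovement, but only a BP_ThirdPersonCharacter receives the fixed, typed damage and sets the Hit flag.
; A Hit event also stops the needle and sets the flag, without dealing damage.
; Once flagged, Tick accumulates time and destroys the actor after a short delay.
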(event `self.ReceiveBeginPlay`)

(event `self.ReceiveActorBeginOverlap`
  (params (OtherActor :type "Actor Object Reference"))
  (set `MovementComponent.Velocity` (0.0 0.0 0.0) (`self.ProjectileMovement`))
  (bind _asbp_third_person_character (cast `/Game/ThirdPerson/Blueprints/BP_ThirdPersonCharacter` OtherActor))
  (`/Game/HPSystem/dmgSystem.doReceiveDamage` _asbp_third_person_character 15.0 "NewEnumerator1" "NewEnumerator2")
  (set `self.hit` true))

(event `self.ReceiveTick`
  (params (DeltaSeconds :type "Float (single-precision)"))
  (if (`self.hit`)
    (set `self.CollisionTime` (+ (`self.CollisionTime`) DeltaSeconds))
    (if (> (`self.CollisionTime`) 1.5)
      (`self.K2_DestroyActor`))))

(event `self.ReceiveHit`
  (params (MyComp :type "PrimitiveComponent Object Reference") (Other :type "Actor Object Reference") (OtherComp :type "PrimitiveComponent Object Reference") (bSelfMoved :type Boolean) (HitLocation :type "Vector Structure") (HitNormal :type "Vector Structure") (NormalImpulse :type "Vector Structure") (Hit :type "HitResult Structure (by ref)"))
  (set `MovementComponent.Velocity` (0.0 0.0 0.0) (`self.ProjectileMovement`))
  (set `self.hit` true))

(fn `UserConstructionScript`)