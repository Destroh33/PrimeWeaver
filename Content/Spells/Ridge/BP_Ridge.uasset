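; BP_Ridge is a spell actor that rises out of the surface it is aimed at.
; On BeginPlay it line-traces forward on Visibility with debug drawing, then moves just below the hit point and keeps only its yaw, or destroys itself next tick on a miss.
; While IsRising is set, Tick lerps it up to the hit point at RiseSpeed, then clears the flag.
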(event `self.ReceiveBeginPlay`
  (bind _returnvalue (`self.K2_GetActorLocation`))
  (bind (_outhit _returnvalue_2) (`KismetSystemLibrary.LineTraceSingle` :`Start` _returnvalue :`End` (+ _returnvalue (* (`self.GetActorForwardVector`) (1000.0 1000.0 1000.0))) :`TraceChannel` "TraceTypeQuery1" :`DrawDebugType` "ForDuration"))
  (if _returnvalue_2
    (bind _output_get (set `self.TargetLocation` (`.Location` (`GameplayStatics.BreakHitResult` _outhit))))
    (bind _output_get_2 (set `self.StartLocation` (`KismetMathLibrary.MakeVector` (.x _output_get) (.y _output_get) (- (.z _output_get) 100.0))))
    (`self.K2_SetActorLocation` _output_get_2)
    (`self.K2_SetActorRotation` (`KismetMathLibrary.MakeRotator` 0.0 0.0 (.yaw (`self.K2_GetActorRotation`))))
    (else
      (`KismetSystemLibrary.DelayUntilNextTick`)
      (`self.K2_DestroyActor`))))

(event `self.ReceiveTick`
  (params (DeltaSeconds :type "Float (single-precision)"))
  (if (`self.isRising`)
    (bind _output_get (set `self.LerpAlpha` (`KismetMathLibrary.FClamp` (+ (`self.LerpAlpha`) (* (`self.RiseSpeed`) DeltaSeconds)))))
    (`self.K2_SetActorLocation` (`KismetMathLibrary.VLerp` (`self.StartLocation`) (`self.TargetLocation`) _output_get))
    (if (>= (`self.LerpAlpha`) 1.0)
      (set `self.isRising` false))))

(fn `UserConstructionScript`)