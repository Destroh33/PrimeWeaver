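; Cauterize is a Tier 2 spell actor that heals the player for half of their missing health.
; On BeginPlay it waits a brief delay, calls DoHeal on the stored player, then attaches the auto-destroying NS_Cauterize Niagara effect to the player's mesh.
; SetPlayer stores the player reference and passes it on to the parent implementation.
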(event `self.ReceiveBeginPlay`
  (bind _player_ref (`self.Player Ref`))
  (`KismetSystemLibrary.Delay` 0.01)
  (bind _health (`/Game/ThirdPerson/Blueprints/BP_ThirdPersonCharacter.getHealth` _player_ref))
  (bind _maxhealth (`/Game/ThirdPerson/Blueprints/BP_ThirdPersonCharacter.getMaxHealth` _player_ref))
  (`/Game/ThirdPerson/Blueprints/BP_ThirdPersonCharacter.doHeal` _player_ref (* (- _maxhealth _health) 0.5))
  (`NiagaraFunctionLibrary.SpawnSystemAttached` "/Game/Spells/Tier2Spells/Cauterize/NS_Cauterize.NS_Cauterize" (`Character.Mesh` _player_ref) "None" (0.0 0.0 0.0) (struct) "KeepRelativeOffset" true))

(fn `SetPlayer`
  (params (PlayerRef :type "/Game/ThirdPerson/Blueprints/BP_ThirdPersonCharacter Object Reference"))
  (bind _output_get (set `self.Player Ref` PlayerRef))
  (`parent.SetPlayer` _output_get))

(fn `UserConstructionScript`)