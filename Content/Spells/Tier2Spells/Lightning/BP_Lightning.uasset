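; BP_Lightning is a Tier 2 lightning spell actor that fires an instant bolt along its forward vector when spawned.
; On BeginPlay it runs a fixed-range visibility line trace from its location.
; The bolt effect's start and end vector parameters follow the trace, ending at the hit point or at maximum range on a miss.
; A hit BP_Enemy receives fixed damage through DoReceiveDamage.
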(event `self.ReceiveBeginPlay`
  (bind _returnvalue (`self.K2_GetActorLocation`))
  (bind _lightningeffect (`self.LightningEffect`))
  (bind _returnvalue_2 (+ (* (`self.GetActorForwardVector`) (1000.0 1000.0 1000.0)) _returnvalue))
  (`NiagaraComponent.SetVariableVec3` _lightningeffect "LightningStart" _returnvalue)
  (bind (_outhit _returnvalue_3) (`KismetSystemLibrary.LineTraceSingle` _returnvalue _returnvalue_2 "TraceTypeQuery1"))
  (if _returnvalue_3
    (bind (_bblockinghit _binitialoverlap _time _distance _location _impactpoint _normal _impactnormal _physmat _hitactor) (`GameplayStatics.BreakHitResult` _outhit))
    (`NiagaraComponent.SetVariableVec3` _lightningeffect "LightningEnd" _location)
    (bind _asbp_enemy (cast `/Game/Characters/Enemy/BP_Enemy` _hitactor))
    (`/Game/Characters/Enemy/BP_Enemy.doReceiveDamage` _asbp_enemy 50.0 "NewEnumerator2" "NewEnumerator2")
    (else
      (`NiagaraComponent.SetVariableVec3` _lightningeffect "LightningEnd" _returnvalue_2))))

(fn `UserConstructionScript`)