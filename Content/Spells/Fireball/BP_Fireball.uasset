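; Fireball spell projectile that explodes on impact and damages spider and moth enemies.
; On BeginPlay it sets its collision sphere as the component driven by ProjectileMovement.
; A sphere hit spawns a Niagara explosion at the impact point, then casts the hit actor to BP_BadSpida or BP_BadMoth to apply fixed damage through DoReceiveDamage.
; The fireball destroys itself after any hit, whether or not it struck an enemy.
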(event `self.ReceiveBeginPlay`
  (`MovementComponent.SetUpdatedComponent` (`self.ProjectileMovement`) (`self.Sphere`)))

(event `self.Sphere.OnComponentHit`
  (params (HitComponent :type "PrimitiveComponent Object Reference") (OtherActor :type "Actor Object Reference") (OtherComp :type "PrimitiveComponent Object Reference") (NormalImpulse :type "Vector Structure") (Hit :type "HitResult Structure (by ref)"))
  (`NiagaraFunctionLibrary.SpawnSystemAtLocation` "/Game/Spells/Fireball/NE_FireBallExplosion_System.NE_FireBallExplosion_System" (`.Location` (`GameplayStatics.BreakHitResult` Hit)))
  (bind _asbp_bad_spida (cast `/Game/Characters/BadSpider/BP_BadSpida` OtherActor)
    (:`then`
      (`/Game/Characters/BadSpider/BP_BadSpida.doReceiveDamage` _asbp_bad_spida 50.0 "NewEnumerator1" "NewEnumerator2"))
    (:`CastFailed`
      (bind _asbp_bad_moth (cast `/Game/Characters/BadMoth/BP_BadMoth` OtherActor)
        (:`then`
          (`/Game/Characters/BadMoth/BP_BadMoth.doReceiveDamage` _asbp_bad_moth 50.0 "NewEnumerator1" "NewEnumerator2"))
        (:`CastFailed`
          _))))
  (`self.K2_DestroyActor`))

(fn `UserConstructionScript`)