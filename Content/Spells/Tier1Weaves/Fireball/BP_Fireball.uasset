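; BP_Fireball is a Tier 1 weave spell projectile that damages enemies with a direct hit and an area explosion.
; ProjectileMovement drives the collision Sphere; on any hit, it spawns the explosion effect and deals full damage if the struck actor is a BP_Enemy.
; A WorldDynamic sphere overlap at the impact then deals lesser splash damage to nearby enemies, excluding the struck actor, before the fireball destroys itself.
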(event `self.ReceiveBeginPlay`
  (`MovementComponent.SetUpdatedComponent` (`self.ProjectileMovement`) (`self.Sphere`)))

(event `self.Sphere.OnComponentHit`
  (params (HitComponent :type "PrimitiveComponent Object Reference") (OtherActor :type "Actor Object Reference") (OtherComp :type "PrimitiveComponent Object Reference") (NormalImpulse :type "Vector Structure") (Hit :type "HitResult Structure (by ref)"))
  (bind (_bblockinghit _binitialoverlap _time _distance _location) (`GameplayStatics.BreakHitResult` Hit))
  (`NiagaraFunctionLibrary.SpawnSystemAtLocation` "/Game/Spells/Tier1Weaves/Fireball/NE_FireBallExplosion_System.NE_FireBallExplosion_System" _location)
  (bind _asbp_enemy (cast `/Game/Characters/Enemy/BP_Enemy` OtherActor)
    (:`then`
      (`/Game/Characters/BadSpider/BP_BadSpida.doReceiveDamage` _asbp_enemy 30.0 "NewEnumerator1" "NewEnumerator2"))
    (:`CastFailed`
      _))
  (bind _outactors (`KismetSystemLibrary.SphereOverlapActors` _location 100.0 (`|MakeArray` "ObjectTypeQuery2" :!type "EObjectTypeQuery Enum") "/Game/Characters/Enemy/BP_Enemy.BP_Enemy_C" (`|MakeArray` OtherActor)))
  (for _array_element _outactors
    (bind _asbp_enemy_2 (cast `/Game/Characters/Enemy/BP_Enemy` _array_element))
    (`/Game/Characters/BadSpider/BP_BadSpida.doReceiveDamage` _asbp_enemy_2 20.0 "NewEnumerator1" "NewEnumerator2"))
  (`self.K2_DestroyActor`))

(fn `UserConstructionScript`)