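; Stream spell actor that heals the player by 15 once and plays a Niagara stream effect that follows them.
; After a brief delay on BeginPlay, it spawns NS_Stream at the player facing forward, with auto-destroy off, then applies the heal.
; Tick keeps the effect on the player's location and facing and re-sets its fixed downward PlayerLocation offset.
; SetPlayer stores the player reference and calls the parent implementation.
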(event `self.ReceiveBeginPlay`
  (bind _player_ref (`self.Player Ref`))
  (`KismetSystemLibrary.Delay` 0.01)
  (bind _returnvalue (`NiagaraFunctionLibrary.SpawnSystemAtLocation` "/Game/Spells/Stream/NS_Stream.NS_Stream" (`self.K2_GetActorLocation` _player_ref) (`KismetMathLibrary.Conv_VectorToRotator` (`self.GetActorForwardVector` _player_ref)) (1.0 1.0 1.0) false))
  (bind _output_get (set `self.Niagara` _returnvalue))
  (`NiagaraComponent.SetNiagaraVariableVec3` _output_get "User.PlayerLocation" (`KismetMathLibrary.MakeVector` 0.0 0.0 -75.0))
  (`/Game/ThirdPerson/Blueprints/BP_ThirdPersonCharacter.doHeal` _player_ref 15.0))

(event `self.ReceiveTick`
  (params (DeltaSeconds :type "Float (single-precision)"))
  (bind _player_ref (`self.Player Ref`))
  (if (`KismetSystemLibrary.IsValid` (`self.Niagara`))
    (`NiagaraComponent.SetNiagaraVariableVec3` (`self.Niagara`) "User.PlayerLocation" (`KismetMathLibrary.MakeVector` 0.0 0.0 -75.0))
    (`SceneComponent.K2_SetWorldLocationAndRotation` (`self.Niagara`) (`self.K2_GetActorLocation` _player_ref) (`KismetMathLibrary.Conv_VectorToRotator` (`self.GetActorForwardVector` _player_ref)) false false)))

(fn `SetPlayer`
  (params (PlayerRef :type "/Game/ThirdPerson/Blueprints/BP_ThirdPersonCharacter Object Reference"))
  (set `self.Player Ref` PlayerRef)
  (`parent.SetPlayer` PlayerRef))

(fn `UserConstructionScript`)