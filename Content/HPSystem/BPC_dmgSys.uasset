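; Damage system component that manages health, death, stuns and timed status effects.
; TakeDamage subtracts health, applies a timed stun for one response type and calls OnDeath at zero, while Heal clamps health to the maximum.
; TakeEffect instantiates an effect class, stores it with context and sends an apply message.
; Tick clears expired stuns and polls game time to send each effect tick and expire messages, removing finished effects.
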(event `self.ReceiveTick`
  (params (DeltaSeconds :type "Float (single-precision)"))
  (bind _returnvalue (`KismetSystemLibrary.GetGameTimeInSeconds`))
  (bind _activeeffects (`self.activeEffects`))
  (if (> (- (`KismetSystemLibrary.GetGameTimeInSeconds`) (`self.lastStunTime`)) (`self.stunLength`))
    (set `self.stunned` false))
  (for (_array_element _array_index) _activeeffects
    (bind (_effectdata _from _to _timestamp _effectinstance _lastticktime) (break `/Game/HPSystem/Effects/S_effectContext` _array_element))
    (if (>= (- _returnvalue _lastticktime) (`/Game/HPSystem/Effects/PDA_effectData.TickRate` _effectdata))
      (message `/Game/HPSystem/Effects/effectInterface.onTick` _effectinstance _array_element)
      (bind _structout (setmembers `/Game/HPSystem/Effects/S_effectContext` :`StructRef` _array_element :`LastTickTime` _returnvalue))
      (`KismetArrayLibrary.Array_Set` _activeeffects _array_index _structout))
    (if (>= (- _returnvalue _timestamp) (`/Game/HPSystem/Effects/PDA_effectData.Duration` _effectdata))
      (message `/Game/HPSystem/Effects/effectInterface.onExpire` _effectinstance _array_element)
      (`KismetArrayLibrary.Array_RemoveItem` _activeeffects _array_element))))

(fn `getEffectClassCount`
  (params (`Effect Class` :type "/Game/HPSystem/Effects/BP_BaseEffect Class Reference"))
  (returns (Count :type Integer))
  (locals (ClassCount :type Integer))
  (set `local.ClassCount` 0)
  (for _array_element (`self.activeEffects`)
    (if (== (`/Game/HPSystem/Effects/PDA_effectData.EffectClass` (`.EffectData_3_208DBBC0D15243D0AD7E94DFCA3D35E7` (break `/Game/HPSystem/Effects/S_effectContext` _array_element))) `Effect Class`)
      (`/Engine/EditorBlueprintResources/StandardMacros.IncrementInt` (`local.ClassCount`))))
  (return (`local.ClassCount`)))

(fn `hasEffectClass`
  (params (EffectClass :type "/Game/HPSystem/Effects/BP_BaseEffect Class Reference"))
  (returns (Result :type Boolean))
  (for _array_element (`self.activeEffects`)
    (if (== (`/Game/HPSystem/Effects/PDA_effectData.EffectClass` (`.EffectData_3_208DBBC0D15243D0AD7E94DFCA3D35E7` (break `/Game/HPSystem/Effects/S_effectContext` _array_element))) EffectClass)
      (return true)))
  (return false))

(fn `heal`
  (params (amount :type "Float (double-precision)"))
  (returns (newHealth :type "Float (double-precision)"))
  (bind _output_get (set `self.health` (`KismetMathLibrary.FClamp` (+ amount (`self.health`)) 0.0 (`self.maxHealth`))))
  (return _output_get))

(fn `takeDamage`
  (params (dmgAmount :type "Float (double-precision)") (dmgResponse :type "/Game/HPSystem/dmgResponse Enum" :default "NewEnumerator0") (dmgType :type "/Game/HPSystem/dmgType Enum" :default "NewEnumerator0") (responseDuration :type "Float (double-precision)"))
  (returns (wasDamaged :type Boolean))
  (if (`self.isAlive`)
    (set `self.stunLength` responseDuration)
    (if (`|EnumEquality` dmgResponse "NewEnumerator2")
      (set `self.stunned` true)
      (set `self.lastStunTime` (`KismetSystemLibrary.GetGameTimeInSeconds`)))
    (bind _output_get (set `self.health` (- (`self.health`) dmgAmount)))
    (if (<= _output_get 0.0)
      (set `self.isAlive` false)
      (`self.onDeath`)
      (return false))
    (else
      (return false))))

(fn `takeEffect`
  (params (EffectData :type "/Game/HPSystem/Effects/PDA_effectData Object Reference") (From :type "Actor Object Reference") (To :type "Actor Object Reference"))
  (bind _returnvalue (`KismetSystemLibrary.GetGameTimeInSeconds`))
  (bind _returnvalue_2 (`|GenericCreateObject` (`/Game/HPSystem/Effects/PDA_effectData.EffectClass` EffectData)))
  (bind _s_effectcontext (make `/Game/HPSystem/Effects/S_effectContext` EffectData From To _returnvalue _returnvalue_2 _returnvalue))
  (`KismetArrayLibrary.Array_Add` (`self.activeEffects`) _s_effectcontext)
  (message `/Game/HPSystem/Effects/effectInterface.onApply` _returnvalue_2 _s_effectcontext))